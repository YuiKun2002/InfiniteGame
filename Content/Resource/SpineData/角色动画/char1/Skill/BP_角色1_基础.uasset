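; Base skill for character 1 that periodically grants flame to the player, scaled by hero level.
; Run derives the interval and flame value from HeroLevel through CalculateRate, mirroring the timer's scaled result around its base.
; Tick counts down, then obtains a flame actor from the resource component, moves it to the player and runs it with that value.
; If no valid flame actor is returned, it adds the value directly through AddFlameNum.
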(event `self.Run`
  (bind ((`HeroLevel` _herolevel)) (break `ItemHeroBase` (`GamePlayer.GetPlayerData` (`self.GetGamePlayer`))))
  (bind _output_get (set `self.Time` (- 30.0 (- (`ItemHeroDataFunc.CalculateRate` 1 _herolevel 1.1 30.0) 30.0))))
  (set `self.TickTime` _output_get)
  (set `self.Value` (`KismetMathLibrary.FTrunc` (`ItemHeroDataFunc.CalculateRate` 1 _herolevel 1.1 25.0))))

(event `self.Tick`
  (params (DeltaTime :type "Float (single-precision) (by ref)"))
  (bind _returnvalue (`self.GetResourceComponent`))
  (if (> (`self.TickTime`) 0.0)
    (set `self.TickTime` (- (`self.TickTime`) DeltaTime))
    (else
      (set `self.TickTime` (`self.Time`))
      (`/Engine/EditorBlueprintResources/StandardMacros.IsValid` _returnvalue
        (:`Is Valid`
          (bind _returnvalue_2 (`ResourceManagerComponent.GetFlame` _returnvalue))
          (`/Engine/EditorBlueprintResources/StandardMacros.IsValid` _returnvalue_2
            (:`Is Valid`
              (`Actor.K2_SetActorLocation` _returnvalue_2 (`Actor.K2_GetActorLocation` (`self.GetGamePlayer`)) false false)
              (`FlameActor.SetFlameValue` _returnvalue_2 (`self.Value`))
              (`FlameActor.Run` _returnvalue_2))
            (:`Is Not Valid`
              (`ResourceManagerComponent.AddFlameNum` _returnvalue (`self.Value`)))))))))