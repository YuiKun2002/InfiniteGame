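; Character 4's third skill, built to deal penetrating damage to ground mice along the map's outer edge.
; Run caches edge cell meshes, but the last-row loop has an empty range, leaving only that row's corners out or unfilled.
; Tick hits cached cells' mice whose GetMouseIsDeath returns true, flagging them hurt.
; As written, the one-second timer decrements by zero, so that pass never fires after Run.
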(event `self.Run`
  (set `self.LauncherTime` 1.0)
  (bind _returnvalue (`MesheControllComponent.GetMapMeshRowAndCol` (`self.GetMesheComponent`)))
  (bind _returnvalue_2 (- (`.Col` (break `Line` _returnvalue)) 1))
  (for _index (range (+ _returnvalue_2 1))
    (bind _returnvalue_3 (`MesheControllComponent.GetMapMouseMesh` (`self.GetMesheComponent`) 0 _index))
    (`KismetArrayLibrary.Array_Add` (`self.Meshe`) _returnvalue_3))
  (for _index_2 (range 0)
    (bind _returnvalue_4 (`MesheControllComponent.GetMapMouseMesh` (`self.GetMesheComponent`) (- (break `Line` _returnvalue) 1) _index_2))
    (`KismetArrayLibrary.Array_Add` (`self.Meshe`) _returnvalue_4))
  (for _index_3 (range 1 (+ (- (break `Line` _returnvalue) 2) 1))
    (bind _returnvalue_5 (`MesheControllComponent.GetMapMouseMesh` (`self.GetMesheComponent`) _index_3 0))
    (`KismetArrayLibrary.Array_Add` (`self.Meshe`) _returnvalue_5)
    (bind _returnvalue_6 (`MesheControllComponent.GetMapMouseMesh` (`self.GetMesheComponent`) _index_3 _returnvalue_2))
    (`KismetArrayLibrary.Array_Add` (`self.Meshe`) _returnvalue_6)))

(event `self.Tick`
  (params (DeltaTime :type "Float (single-precision) (by ref)"))
  (bind _launchertime (`self.LauncherTime`))
  (if (> _launchertime 0.0)
    (set `self.LauncherTime` (- _launchertime 0.0))
    (else
      (set `self.LauncherTime` 1.0)
      (for _array_element (`self.Meshe`)
        (bind _values (`BlueprintMapLibrary.Map_Values` (`MapMouseMesheManager.GetCurMouseCopy` _array_element)))
        (for _array_element_2 _values
          (`/Engine/EditorBlueprintResources/StandardMacros.IsValid` _array_element_2
            (:`Is Valid`
              (bind _returnvalue (`MouseActor.GetMouseIsDeath` _array_element_2))
              (if _returnvalue
                (bind _returnvalue_2 (`MouseActor.GetMouseLineType` _array_element_2))
                (if (`|EnumEquality` _returnvalue_2 "OnGround")
                  (bind _returnvalue_3 (`MouseActor.BeHit` _array_element_2 (`self.GetGamePlayer`) 10.0 "Panetrate"))
                  (if _returnvalue_3
                    (`MouseActor.SetbIsHurt` _array_element_2 true)))))))))))