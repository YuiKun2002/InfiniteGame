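; Skill 1 of character 4: a timed auto-attack that strikes a ground or sky mouse enemy in the player's row.
; Run scales attack and cooldown from hero level, registers a pooled super-weapon bullet and debug-prints the cooldown.
; When the Tick countdown expires, it moves the bullet onto the found target and calls the hit overlap directly.
; It also gives that target a one-second lifespan.
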(event `self.Run`
  (bind ((`HeroLevel` _herolevel)) (break `ItemHeroBase` (`GamePlayer.GetPlayerData` (`self.GetGamePlayer`))))
  (bind _returnvalue (- 9.5 (- (`ItemHeroDataFunc.CalculateRate` 1 _herolevel 1.005 9.5) 9.5)))
  (set `self.Attack` (`ItemHeroDataFunc.CalculateRate` 1 _herolevel 1.01 15.0))
  (set `self.LauncherTime` _returnvalue)
  (bind _output_get (set `self.NewVar_0` _returnvalue))
  (`GamePlayerSuperWeapon.AddNewBullet` (`GamePlayer.GetPlayerSuperWeapon` (`self.GetGamePlayer`)) "bb" (`self.Res Path`) 1)
  (`KismetSystemLibrary.PrintString` null (`KismetStringLibrary.Conv_DoubleToString` _output_get) true true (struct :`G` 0.66 :`B` 1.0 :`A` 1.0) 5.0))

(event `self.Tick`
  (params (DeltaTime :type "Float (single-precision) (by ref)"))
  (bind _bu (`self.Bu`))
  (bind _alien (`self.Alien`))
  (bind _launchertime (`self.LauncherTime`))
  (bind _alien_2 (`self.Alien`))
  (bind _returnvalue_row (break `Line` (`GamePlayer.GetLine` (`self.GetGamePlayer`))))
  (if (> _launchertime 0.0)
    (set `self.LauncherTime` (- _launchertime DeltaTime))
    (else
      (set `self.LauncherTime` (`self.NewVar_0`))
      (bind _returnvalue (`GameSystemFunction.LockingAttackComponentCheckAlien` (`self.GetMouseManager`) _returnvalue_row (`|MakeSet` "E_MouseGround" "E_MouseSky" :!type "ELineTraceType Enum")))
      (`/Engine/EditorBlueprintResources/StandardMacros.IsValid` _returnvalue
        (:`Is Valid`
          (set `self.Bu` (`GamePlayerSuperWeapon.GetBulletByTag` (`GamePlayer.GetPlayerSuperWeapon` (`self.GetGamePlayer`)) "bb"))
          (set `self.Alien` _returnvalue)
          (`Actor.K2_SetActorLocation` (`self.Bu`) (`Actor.K2_GetActorLocation` _alien_2) false false)
          (`FlyItemActor.SetObjectActorLocation` _bu _alien_2)
          (`FlyItemActor.SetATK` _bu (`self.Attack`))
          (`FlyItemActor.SetFloatModeEnable` _bu true)
          (`FlyItemActor.Init` _bu)
          (`FlyItemActor.HitMouse_OverlapBegin` (`self.Bu`) _alien)
          (`Actor.SetLifeSpan` _alien 1.0))))))