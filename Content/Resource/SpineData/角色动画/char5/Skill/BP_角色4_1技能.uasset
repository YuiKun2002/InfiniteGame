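; Super-weapon skill for character 5 that periodically strikes a locked-on ground or air enemy.
; Run scales damage up and cooldown down with hero level, registers the "bb" bullet pool and removes bullet "aa".
; When the timer expires, Tick places a bullet on a target in the player's row and triggers its hit directly.
; A successful strike queues a brief follow-up targeting with row 0, then the full cooldown resumes.
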(event `self.Run`
  (bind _returnvalue (`GamePlayer.GetPlayerSuperWeapon` (`self.GetGamePlayer`)))
  (bind ((`HeroLevel` _herolevel)) (break `ItemHeroBase` (`GamePlayer.GetPlayerData` (`self.GetGamePlayer`))))
  (bind _returnvalue_2 (- 9.0 (- (`ItemHeroDataFunc.CalculateRate` 1 _herolevel 1.005 9.0) 9.0)))
  (set `self.Attack` (`ItemHeroDataFunc.CalculateRate` 1 _herolevel 1.01 15.0))
  (set `self.LauncherTime` _returnvalue_2)
  (set `self.NewVar_0` _returnvalue_2)
  (`GamePlayerSuperWeapon.AddNewBullet` _returnvalue "bb" (`self.Res Path`) 1)
  (set `self.bP` false)
  (`GamePlayerSuperWeapon.RemoveBulletByTag` _returnvalue "aa"))

(event `self.Tick`
  (params (DeltaTime :type "Float (single-precision) (by ref)"))
  (bind _bu (`self.Bu`))
  (bind _launchertime (`self.LauncherTime`))
  (bind _alien (`self.Alien`))
  (bind _alien_2 (`self.Alien`))
  (bind _bu_2 (`self.Bu`))
  (bind _returnvalue_row (break `Line` (`GamePlayer.GetLine` (`self.GetGamePlayer`))))
  (if (> _launchertime 0.0)
    (set `self.LauncherTime` (- _launchertime DeltaTime))
    (else
      (set `self.LauncherTime` (`self.NewVar_0`))
      (if (`self.bP`)
        (set `self.bP` false)
        (bind _returnvalue (`GameSystemFunction.LockingAttackComponentCheckAlien` (`self.GetMouseManager`) 0 (`|MakeSet` "E_MouseGround" "E_MouseSky" :!type "ELineTraceType Enum")))
        (`/Engine/EditorBlueprintResources/StandardMacros.IsValid` _returnvalue
          (:`Is Valid`
            (set `self.Bu` (`GamePlayerSuperWeapon.GetBulletByTag` (`GamePlayer.GetPlayerSuperWeapon` (`self.GetGamePlayer`)) "bb"))
            (set `self.Alien` _returnvalue)
            (`Actor.K2_SetActorLocation` (`self.Bu`) (`Actor.K2_GetActorLocation` _alien) false false)
            (`FlyItemActor.SetObjectActorLocation` _bu _alien)
            (`FlyItemActor.SetATK` _bu (`self.Attack`))
            (`FlyItemActor.SetFloatModeEnable` _bu true)
            (`FlyItemActor.Init` _bu)
            (`FlyItemActor.HitMouse_OverlapBegin` (`self.Bu`) (`self.Alien`))))
        (else
          (bind _returnvalue_2 (`GameSystemFunction.LockingAttackComponentCheckAlien` (`self.GetMouseManager`) _returnvalue_row (`|MakeSet` "E_MouseGround" "E_MouseSky" :!type "ELineTraceType Enum")))
          (`/Engine/EditorBlueprintResources/StandardMacros.IsValid` _returnvalue_2
            (:`Is Valid`
              (set `self.Bu` (`GamePlayerSuperWeapon.GetBulletByTag` (`GamePlayer.GetPlayerSuperWeapon` (`self.GetGamePlayer`)) "bb"))
              (set `self.Alien` _returnvalue_2)
              (`Actor.K2_SetActorLocation` (`self.Bu`) (`Actor.K2_GetActorLocation` _alien_2) false false)
              (`FlyItemActor.SetObjectActorLocation` _bu_2 _alien_2)
              (`FlyItemActor.SetATK` _bu_2 (`self.Attack`))
              (`FlyItemActor.SetFloatModeEnable` _bu_2 true)
              (`FlyItemActor.Init` _bu_2)
              (`FlyItemActor.HitMouse_OverlapBegin` (`self.Bu`) (`self.Alien`))
              (set `self.LauncherTime` 0.3)
              (set `self.bP` true))))))))