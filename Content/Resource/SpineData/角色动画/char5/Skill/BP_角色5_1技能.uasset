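; Character 5_1 skill that plays its configured card on three vertically adjacent cells, three columns offset from the player.
; GetPointP bounds-checks each cell against the map grid and reads its terrain type, skipping invalid cells.
; Water and magma cells first receive a terrain-specific card from a local variable, then the main card.
; Placement is issued as "/game play" command strings, with each card's grade looked up by name.
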(event `self.Run`
  (`self.GetPoint` (`self.Card Name`) 0 3)
  (`self.GetPoint` (`self.Card Name`) 1 3)
  (`self.GetPoint` (`self.Card Name`) -1 3))

(fn `GetPoint`
  (params (CardName :type Text) (RowOffset :type Integer) (ColOffset :type Integer))
  (locals (NewLocalVar_0 :type Text :default "NSLOCTEXT(\"\", \"1E9DDE0744FA06A6143E46A017BF72E9\", \"冰片\")") (NewLocalVar_1 :type Text :default "NSLOCTEXT(\"\", \"3FAFFBB24ED3847DED9C75B090AEC4AE\", \"橙片\")"))
  (bind _newlocalvar_1 (`local.NewLocalVar_1`))
  (bind _newlocalvar_0 (`local.NewLocalVar_0`))
  (bind _output_get (set `self.TargetGrade` (`CardManagerComponent.GetCardGradeByName` (`self.GetCardComponent`) CardName)))
  (bind (_overline _linetype _outline) (`self.GetPointP` RowOffset ColOffset))
  (if _overline
    (return)
    (elif (`|EnumEquality` _linetype "OnWater")
      (`|ExecutionSequence`
        (:`then_0`
          (`GameSystemFunction.AddGameinstructions` (`self.GetGamePlayer`) (`KismetStringLibrary.Concat_StrStr` "/game play " (`KismetTextLibrary.Conv_TextToString` _newlocalvar_1) "," (`KismetStringLibrary.Conv_IntToString` (`CardManagerComponent.GetCardGradeByName` (`self.GetCardComponent`) _newlocalvar_1)) " " (`KismetStringLibrary.Conv_IntToString` (break `Line` _outline)) "," (`KismetStringLibrary.Conv_IntToString` (`.Col` (break `Line` _outline)))) false))
        (:`then_1`
          (bind _returnvalue (`KismetStringLibrary.Concat_StrStr` "/game play " (`KismetTextLibrary.Conv_TextToString` CardName) "," (`KismetStringLibrary.Conv_IntToString` _output_get) " " (`KismetStringLibrary.Conv_IntToString` (break `Line` _outline)) "," (`KismetStringLibrary.Conv_IntToString` (`.Col` (break `Line` _outline)))))
          (`GameSystemFunction.AddGameinstructions` (`self.GetGamePlayer`) _returnvalue false)))
      (elif (`|EnumEquality` _linetype "Magma")
        (`|ExecutionSequence`
          (:`then_0`
            (`GameSystemFunction.AddGameinstructions` (`self.GetGamePlayer`) (`KismetStringLibrary.Concat_StrStr` "/game play " (`KismetTextLibrary.Conv_TextToString` _newlocalvar_0) "," (`KismetStringLibrary.Conv_IntToString` (`CardManagerComponent.GetCardGradeByName` (`self.GetCardComponent`) _newlocalvar_0)) " " (`KismetStringLibrary.Conv_IntToString` (break `Line` _outline)) "," (`KismetStringLibrary.Conv_IntToString` (`.Col` (break `Line` _outline)))) false))
          (:`then_1`
            (`GameSystemFunction.AddGameinstructions` (`self.GetGamePlayer`) _returnvalue false)))
        (else
          (`GameSystemFunction.AddGameinstructions` (`self.GetGamePlayer`) _returnvalue false))))))

(fn `GetPointP`
  (params (RowOffset :type Integer) (ColOffset :type Integer))
  (returns (OverLine :type Boolean) (LineType :type "ELineType Enum") (OutLine :type "Line Structure"))
  (bind (_returnvalue_row _returnvalue_col) (break `Line` (`GamePlayer.GetLine` (`self.GetGamePlayer`))))
  (bind _returnvalue (+ _returnvalue_row RowOffset))
  (bind _returnvalue_2 (+ _returnvalue_col ColOffset))
  (bind _returnvalue_3 (`MesheControllComponent.GetMapMeshRowAndCol` (`self.GetMesheComponent`)))
  (if (or (< _returnvalue 0) (>= _returnvalue (break `Line` _returnvalue_3)))
    (return true "OnGround")
    (elif (or (< _returnvalue_2 0) (>= _returnvalue_2 (`.Col` (break `Line` _returnvalue_3))))
      (return true "OnGround")
      (else
        (bind _returnvalue_4 (`MesheControllComponent.GetMapMesh` (`self.GetMesheComponent`) _returnvalue _returnvalue_2))
        (`/Engine/EditorBlueprintResources/StandardMacros.IsValid` _returnvalue_4
          (:`Is Valid`
            (bind _returnvalue_5 (`MapMeshe.GetUIMapMeshe` _returnvalue_4))
            (`/Engine/EditorBlueprintResources/StandardMacros.IsValid` _returnvalue_5
              (:`Is Valid`
                (return false (`UI_MapMeshe.M_ELineType` _returnvalue_5) (make `Line` _returnvalue _returnvalue_2)))
              (:`Is Not Valid`
                (return true "OnGround"))))
          (:`Is Not Valid`
            (return true "OnGround")))))))