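; Basic skill for character 5 that periodically fires a bullet from the player's position in the player's current row.
; On Run it scales attack and firing interval from hero level, with the interval shrinking as level rises, and registers a one-slot bullet pool on the player's super weapon.
; Tick counts down the timer, then resets it and initializes the pooled bullet with row, location, attack and float mode.
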(event `self.Run`
  (bind ((`HeroLevel` _herolevel)) (break `ItemHeroBase` (`GamePlayer.GetPlayerData` (`self.GetGamePlayer`))))
  (bind _returnvalue (- 23.0 (- (`ItemHeroDataFunc.CalculateRate` 1 _herolevel 1.01 23.0) 23.0)))
  (set `self.Attack` (`ItemHeroDataFunc.CalculateRate` 1 _herolevel 1.08 5.0))
  (set `self.LauncherTime` _returnvalue)
  (set `self.NewVar_0` _returnvalue)
  (`GamePlayerSuperWeapon.AddNewBullet` (`GamePlayer.GetPlayerSuperWeapon` (`self.GetGamePlayer`)) "aa" (`self.Res Path`) 1))

(event `self.Tick`
  (params (DeltaTime :type "Float (single-precision) (by ref)"))
  (bind _returnvalue (`self.GetGamePlayer`))
  (bind _newvar_1 (`self.NewVar_1`))
  (bind _launchertime (`self.LauncherTime`))
  (bind _returnvalue_row (break `Line` (`GamePlayer.GetLine` _returnvalue)))
  (if (> _launchertime 0.0)
    (set `self.LauncherTime` (- _launchertime DeltaTime))
    (else
      (set `self.LauncherTime` (`self.NewVar_0`))
      (bind _output_get (set `self.NewVar_1` (`GamePlayerSuperWeapon.GetBulletByTag` (`GamePlayer.GetPlayerSuperWeapon` (`self.GetGamePlayer`)) "aa")))
      (`/Engine/EditorBlueprintResources/StandardMacros.IsValid` _output_get
        (:`Is Valid`
          (`FlyItemActor.SetLine` _newvar_1 _returnvalue_row)
          (`Actor.K2_SetActorLocation` _newvar_1 (`Actor.K2_GetActorLocation` _returnvalue) false false)
          (`FlyItemActor.SetATK` _newvar_1 (`self.Attack`))
          (`FlyItemActor.SetFloatModeEnable` _newvar_1 true)
          (`FlyItemActor.Init` _newvar_1))))))