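; Character 3's second skill, a card skill commented as a 100% HP increase for the defence type.
; Run writes the DefenceCardHPRate variable to the card component's dynamic property, then calls ChangeProperty to update it.
; Tick overwrites that rate with a random float from a fixed range and reapplies it on each call, so the bonus does not stay at a fixed 100%.
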(event `self.Run`
  (bind _returnvalue (`self.GetCardComponent`))
  ;[1 1 1] 生命值增加100%   （防御系）
  (`/Engine/EditorBlueprintResources/StandardMacros.IsValid` _returnvalue
    (:`Is Valid`
      (`self.SetFloatProperty` (`CardManagerComponent.GetDynamicProperty` _returnvalue) "DefenceCardHPRate" (`self.DefenceCardHPRate`))
      (`CardManagerComponent.ChangeProperty` _returnvalue))))

(event `self.Tick`
  (params (DeltaTime :type "Float (single-precision) (by ref)"))
  (bind _returnvalue (`self.GetCardComponent`))
  (`/Engine/EditorBlueprintResources/StandardMacros.IsValid` _returnvalue
    (:`Is Valid`
      (set `self.DefenceCardHPRate` (`KismetMathLibrary.RandomFloatInRange` 1.0 10.0))
      (`self.SetFloatProperty` (`CardManagerComponent.GetDynamicProperty` _returnvalue) "DefenceCardHPRate" (`self.DefenceCardHPRate`))
      (`CardManagerComponent.ChangeProperty` _returnvalue))))