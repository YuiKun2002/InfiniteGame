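; Basic skill Blueprint for a hero character that repeatedly attacks ground aliens on a one-second countdown.
; On Run, it derives attack power from the player's hero level through a rate calculation and arms the timer.
; Tick counts the timer down, then resets it and calls a map-mouse-manager range hit using the player's line, that attack value and the mesh component.
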(event `self.Run`
  (set `self.Attack` (`KismetMathLibrary.FTrunc` (`ItemHeroDataFunc.CalculateRate` 1 (`.HeroLevel` (break `ItemHeroBase` (`GamePlayer.GetPlayerData` (`self.GetGamePlayer`)))) 1.01 2.0)))
  (set `self.LauncherTime` 1.0))

(event `self.Tick`
  (params (DeltaTime :type "Float (single-precision) (by ref)"))
  (bind _launchertime (`self.LauncherTime`))
  (if (> _launchertime 0.0)
    (set `self.LauncherTime` (- _launchertime DeltaTime))
    (else
      (set `self.LauncherTime` 1.0)
      (`GameSystemFunction.PlayerHitRangeAlienByMapMouseManager` (`GamePlayer.GetLine` (`self.GetGamePlayer`)) 1 (struct) "OnGround" (`KismetMathLibrary.Conv_IntToDouble` (`self.Attack`)) (`self.GetMesheComponent`)))))