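; Skill 3 Blueprint for character 3, which periodically fires a bullet through the player's super weapon.
; Run registers a single-bullet pool from the resource path and starts an 18-second countdown.
; On Tick, each expiry resets the countdown and fetches the tagged bullet.
; The bullet is placed at the player, aimed via the player's current mouse, given the player's line row, then initialized with zero attack and float mode off.
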(event `self.Run`
  (`GamePlayerSuperWeapon.AddNewBullet` (`GamePlayer.GetPlayerSuperWeapon` (`self.GetGamePlayer`)) "a" (`self.Res Path`) 1)
  (set `self.LauncherTime` 18.0))

(event `self.Tick`
  (params (DeltaTime :type "Float (single-precision) (by ref)"))
  (bind _returnvalue (`self.GetGamePlayer`))
  (bind _bullet (`self.Bullet`))
  (bind _bullet_2 (`self.Bullet`))
  (bind _returnvalue_row (break `Line` (`GamePlayer.GetLine` (`self.GetGamePlayer`))))
  (bind _returnvalue_2 (`GamePlayerSuperWeapon.GetBulletByTag` (`GamePlayer.GetPlayerSuperWeapon` (`self.GetGamePlayer`)) "a"))
  (if (> (`self.LauncherTime`) 0.0)
    (set `self.LauncherTime` (- (`self.LauncherTime`) DeltaTime))
    (else
      (set `self.LauncherTime` 18.0)
      (`/Engine/EditorBlueprintResources/StandardMacros.IsValid` _returnvalue_2
        (:`Is Valid`
          (set `self.Bullet` _returnvalue_2)
          (`FlyItemActor.SetFlyParentActor` _bullet_2 _returnvalue)
          (`Actor.K2_SetActorLocation` _bullet_2 (`Actor.K2_GetActorLocation` _returnvalue) false false)
          (bind _returnvalue_3 (`GamePlayer.GetCurrentMouse` _returnvalue))
          (`FlyItemActor.SetObjectActorLocation` _bullet_2 _returnvalue_3)
          (`FlyItemActor.SetLine` _bullet _returnvalue_row)
          (`FlyItemActor.SetFloatModeEnable` _bullet false)
          (`FlyItemActor.SetATK` _bullet 0.0)
          (`FlyItemActor.Init` _bullet))))))