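; Basic skill Blueprint for character 3 that periodically applies an HP boost to cards on grid cells around the player's line.
; On Run, it scales the boost by hero level and caches the map UI widgets in a generated cell matrix.
; Tick counts down a one-second timer, then updates the state of each card matching the ID in those cells, passing the computed Attack value as the HP increase.
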(event `self.Run`
  (set `self.Attack` (`ItemHeroDataFunc.CalculateRate` 1 (`.HeroLevel` (break `ItemHeroBase` (`GamePlayer.GetPlayerData` (`self.GetGamePlayer`)))) 1.01 2.0))
  (set `self.LauncherTime` 1.0)
  ;[1 1 1] 初始化检测范围
  (for _array_element (`GameSystemFunction.GenerateMatrixByPoint` (`self.GetMesheComponent`) (`GamePlayer.GetLine` (`self.GetGamePlayer`)) 1)
    (bind _returnvalue (`MesheControllComponent.GetMesh` (`self.GetMesheComponent`) (break `Line` _array_element) (`.Col` (break `Line` _array_element))))
    (bind _returnvalue_2 (`MapMeshe.GetUIMapMeshe` _returnvalue))
    (`/Engine/EditorBlueprintResources/StandardMacros.IsValid` _returnvalue_2
      (:`Is Valid`
        (`KismetArrayLibrary.Array_Add` (`self.UIs`) _returnvalue_2)))))

(event `self.Tick`
  (params (DeltaTime :type "Float (single-precision) (by ref)"))
  (bind _launchertime (`self.LauncherTime`))
  (if (> _launchertime 0.0)
    (set `self.LauncherTime` (- _launchertime DeltaTime))
    (else
      (set `self.LauncherTime` 1.0)
      (for _array_element (`self.UIs`)
        (`/Engine/EditorBlueprintResources/StandardMacros.IsValid` _array_element
          (:`Is Valid`
            (bind _returnvalue (`UI_MapMeshe.GetCardByID` _array_element (`self.ID`)))
            (`/Engine/EditorBlueprintResources/StandardMacros.IsValid` _returnvalue
              (:`Is Valid`
                (`CardActor.UpdateCardState` _returnvalue (`self.ATK Value_0`) (`self.Attack`))))))))))