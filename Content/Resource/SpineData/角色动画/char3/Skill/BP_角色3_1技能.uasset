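; Character 3's first skill, an aura that gives damage reduction to cards on map cells near the player.
; Run builds the affected area once from the player's line with GenerateMatrixByPoint and caches each valid cell's UI map mesh.
; Tick uses a countdown, starting immediately and repeating every two seconds, to reapply the damage-reduction buff to every valid card in those cells, with the player as source.
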(event `self.Run`
  (set `self.LauncherTime` 0.0)
  ;[1 1 1] 初始化检测范围
  (for _array_element (`GameSystemFunction.GenerateMatrixByPoint` (`self.GetMesheComponent`) (`GamePlayer.GetLine` (`self.GetGamePlayer`)) 1)
    (bind _returnvalue (`MesheControllComponent.GetMesh` (`self.GetMesheComponent`) (break `Line` _array_element) (`.Col` (break `Line` _array_element))))
    (bind _returnvalue_2 (`MapMeshe.GetUIMapMeshe` _returnvalue))
    (`/Engine/EditorBlueprintResources/StandardMacros.IsValid` _returnvalue_2
      (:`Is Valid`
        (`KismetArrayLibrary.Array_Add` (`self.UIs`) _returnvalue_2)))))

(event `self.Tick`
  (params (DeltaTime :type "Float (single-precision) (by ref)"))
  (bind _launchertime (`self.LauncherTime`))
  (if (> _launchertime 0.0)
    (set `self.LauncherTime` (- _launchertime DeltaTime))
    (else
      (set `self.LauncherTime` 2.0)
      (for _array_element (`self.UIs`)
        (bind _values (`BlueprintMapLibrary.Map_Values` (`UI_MapMeshe.M_Card_Data` _array_element)))
        (for _array_element_2 _values
          (`/Engine/EditorBlueprintResources/StandardMacros.IsValid` _array_element_2
            (:`Is Valid`
              (`CardActor.ParseBuff_Information` _array_element_2 (make `GameBuffInfor` (`|MakeMap` "DamageRedu" 2.0 :!type "EGameBuffTag Enum" :!valuetype "Float (single-precision)") (`|MakeMap` "DamageRedu" "/Game/Resource/SpineData/角色动画/char3/Skill/BP_伤害减免Buff_0_5_Card.BP_伤害减免Buff_0_5_Card_C" :!type "EGameBuffTag Enum" :!valuetype "BuffDynamicProperty Class Reference")) (`self.GetGamePlayer`)))))))))