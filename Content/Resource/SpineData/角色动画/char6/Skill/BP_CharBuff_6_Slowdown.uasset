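; Slowdown buff for character 6 that derives its slow rate from the hero's level when initialized by that character's base skill.
; On init it caches the skill, reads the player's hero level and mirrors CalculateRate's growth around the base value, so Rate falls as level rises, clamped to a minimum.
; The result is stored in Rate and printed for debugging; this graph does not apply the slow itself.
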(event `self.OnDefObjectInit`
  (params (Value :type "Object Object Reference"))
  (bind `_asbp_角色6_基础技能` (cast `/Game/Resource/SpineData/角色动画/char6/Skill/BP_角色6_基础技能` Value))
  (bind _output_get (set `self.As BP 角色6 基础技能` `_asbp_角色6_基础技能`))
  (bind _output_get_2 (set `self.Rate` (- 0.9 (- (`ItemHeroDataFunc.CalculateRate` 1 (`.HeroLevel` (break `ItemHeroBase` (`GamePlayer.GetPlayerData` (`GamePlayerSkillObject.GetGamePlayer` _output_get)))) 1.01 0.9) 0.9))))
  (if (<= _output_get_2 0.4)
    (set `self.Rate` 0.4))
  (`KismetSystemLibrary.PrintString` null (`KismetStringLibrary.Conv_DoubleToString` (`self.Rate`))))