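; Character 6's basic skill, a periodic area slow that debuffs mice on nearby map grid cells.
; On Run, it generates a cell matrix from its mesh component and the player's line, then caches the valid map cells.
; Tick uses a one-second countdown to apply a short SlowDown buff, via BP_CharBuff_6_Slowdown, to every living mouse currently in those cells.
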(event `self.Run`
  (set `self.LauncherTime` 0.0)
  ;[1 1 1] 初始化检测范围
  (for _array_element (`GameSystemFunction.GenerateMatrixByPoint` (`self.GetMesheComponent`) (`GamePlayer.GetLine` (`self.GetGamePlayer`)) 2)
    (bind _returnvalue (`MesheControllComponent.GetMapMouseMesh` (`self.GetMesheComponent`) (break `Line` _array_element) (`.Col` (break `Line` _array_element))))
    (`/Engine/EditorBlueprintResources/StandardMacros.IsValid` _returnvalue
      (:`Is Valid`
        (`KismetArrayLibrary.Array_Add` (`self.UIs`) _returnvalue)))))

(event `self.Tick`
  (params (DeltaTime :type "Float (single-precision) (by ref)"))
  (bind _launchertime (`self.LauncherTime`))
  (if (> _launchertime 0.0)
    (set `self.LauncherTime` (- _launchertime DeltaTime))
    (else
      (set `self.LauncherTime` 1.0)
      (for _array_element (`self.UIs`)
        (`/Engine/EditorBlueprintResources/StandardMacros.IsValid` _array_element
          (:`Is Valid`
            (bind _values (`BlueprintMapLibrary.Map_Values` (`MapMouseMesheManager.GetCurMouseCopy` _array_element)))
            (for _array_element_2 _values
              (`/Engine/EditorBlueprintResources/StandardMacros.IsValid` _array_element_2
                (:`Is Valid`
                  (bind _returnvalue (`MouseActor.GetMouseIsDeath` _array_element_2))
                  (if (not _returnvalue)
                    (`MouseActor.ParseBuff_Information` _array_element_2 (make `GameBuffInfor` (`|MakeMap` "SlowDown" 1.1 :!type "EGameBuffTag Enum" :!valuetype "Float (single-precision)") (`|MakeMap` "SlowDown" "/Game/Resource/SpineData/角色动画/char6/Skill/BP_CharBuff_6_Slowdown.BP_CharBuff_6_Slowdown_C" :!type "EGameBuffTag Enum" :!valuetype "BuffDynamicProperty Class Reference")) self)))))))))))