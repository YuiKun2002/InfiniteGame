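; Character 6's first skill, which periodically freezes a random enemy mouse.
; Tick runs a 14-second cooldown, then gathers lines that contain mice and picks one at random.
; A mouse from that line receives a five-second Freeze buff via ParseBuffInformation, attributed to the game player.
; Random is re-evaluated at each use, so the validity check, death check and buff can hit different mice.
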(event `self.Run`
  (set `self.LauncherTime` 14.0))

(event `self.Tick`
  (params (DeltaTime :type "Float (single-precision) (by ref)"))
  (bind _returnvalue (`self.GetMouseManager`))
  (bind _launchertime (`self.LauncherTime`))
  (if (> _launchertime 0.0)
    (set `self.LauncherTime` (- _launchertime DeltaTime))
    (else
      (set `self.LauncherTime` 14.0)
      (`KismetArrayLibrary.Array_Clear` (`self.IndexList`))
      (for _index (range (`MouseManagerComponent.GetLineCount` _returnvalue))
        (bind _returnvalue_2 (`MouseManagerComponent.GetMouseLineManager` _returnvalue _index))
        (if (`MouseLineManager.GetMouseExist` _returnvalue_2)
          (`KismetArrayLibrary.Array_Add` (`self.IndexList`) _index)))
      (if (> (`KismetArrayLibrary.Array_Length` (`self.IndexList`)) 0)
        (bind _returnvalue_3 (`MouseManagerComponent.GetMouseLineManager` _returnvalue (`KismetArrayLibrary.Array_Random` (`self.IndexList`))))
        (bind _values (`BlueprintMapLibrary.Map_Values` (`MouseLineManager.GetMouseAll` _returnvalue_3)))
        (bind _outitem (`KismetArrayLibrary.Array_Random` _values))
        (`/Engine/EditorBlueprintResources/StandardMacros.IsValid` _outitem
          (:`Is Valid`
            (bind _returnvalue_4 (`MouseActor.GetMouseIsDeath` _outitem))
            (if (not _returnvalue_4)
              (`MouseActor.ParseBuff_Information` _outitem (make `GameBuffInfor` (`|MakeMap` "Freeze" 5.0 :!type "EGameBuffTag Enum" :!valuetype "Float (single-precision)") (`|MakeMap` "Freeze" "/Game/Resource/SpineData/角色动画/char6/Skill/BP_角色6_1技能buff能力.BP_角色6_1技能buff能力_C" :!type "EGameBuffTag Enum" :!valuetype "BuffDynamicProperty Class Reference")) (`self.GetGamePlayer`)))))))))