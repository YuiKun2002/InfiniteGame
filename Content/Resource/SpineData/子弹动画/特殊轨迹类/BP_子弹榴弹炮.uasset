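; Howitzer bullet Blueprint (榴弹炮, special-trajectory class) that creates an area bomb on the game's grid.
; On BeginPlay it binds a custom event to the parent's spawn event.
; That event builds a bomb from the bullet's line and column, extended one cell in each direction, passing its current attack and buff.
; The bomb targets ground mice and uses the extensible flame generator (BP_延展性火焰生成器) as its extra visual.
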(event `self.ReceiveBeginPlay`
  (`parent.ReceiveBeginPlay`)
  (add `self.OnSpwanEvent` (delegate `CustomEvent_1`)))

(event `CustomEvent_1`
  (bind _returnvalue (`self.GetLine`))
  (bind _returnvalue_2 (`self.GetCurATK`))
  (bind _returnvalue_3 (`self.GetBuff`))
  (`CardFunctionBombBase.CreateBombGridExtensionFunction` self "/Game/Resource/SpineData/其他动画/火焰/火焰生成器/BP_延展性火焰生成器.BP_延展性火焰生成器_C" (make `Line` _returnvalue (`self.Col`)) (make `CardFunctionBomb_GridExtension_ImplementTRB` 1 1 1 1) (`|MakeArray` "MouseGround" :!type "EMouseCollisionType Enum") _returnvalue_3 _returnvalue_2))

(fn `UserConstructionScript`
  (`parent.UserConstructionScript`))