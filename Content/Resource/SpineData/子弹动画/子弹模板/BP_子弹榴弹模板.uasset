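; Template Blueprint for a pooled, Spine-animated grenade (榴弹) projectile that lobs onto a map grid cell.
; On init it loops its default animation while an Up timeline lifts it vertically, then snaps its Y to the target cell from the map's mesh controller.
; A Down timeline drops it onto that cell and fires the spawn event.
; It returns to the pool immediately, or after the optional end animation completes.
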(event `self.ReceiveBeginPlay`
  (`self.InitSpineShow`))

(event `self.OnInit`
  (bind (_returnvalue_x _returnvalue_y _returnvalue_z) (`KismetMathLibrary.BreakVector` (`self.K2_GetActorLocation`)))
  (`SpineSkeletonAnimationComponent.SetAnimation` (`self.AnimComp`) 0 "Def" true)
  (set `self.CurLocation` (`self.K2_GetActorLocation`))
  (bind (_direction _newtrack_0) (`Timeline|Up` :!via `PlayFromStart`)
    (:`Update`
      (`self.K2_SetActorLocation` (`KismetMathLibrary.VLerp` (`self.CurLocation`) (+ (`self.CurLocation`) (0.0 0.0 400.0)) _newtrack_0)))
    (:`Finished`
      (bind _returnvalue (`GameMapInstance.GetGameMapInstance`))
      (bind _returnvalue_2 (`GameMapInstance.GetMesheControllComponent` _returnvalue))
      (bind _returnvalue_3 (`self.GetLine`))
      (bind _returnvalue_4 (`MesheControllComponent.GetMapMeshLocation` _returnvalue_2 _returnvalue_3 (`self.Col`)))
      (set `self.TargetLocation_0` (`KismetMathLibrary.MakeVector` (.x _returnvalue_4) (.y _returnvalue_4) (.z _returnvalue_4)))
      (`self.K2_SetActorLocation` (`KismetMathLibrary.MakeVector` _returnvalue_x (.y _returnvalue_4) _returnvalue_z))
      (set `self.CurLocation` (`self.K2_GetActorLocation`))
      (bind (_direction_2 _newtrack_0_2) (`Timeline|Down` :!via `PlayFromStart`)
        (:`Update`
          (`self.K2_SetActorLocation` (`KismetMathLibrary.VLerp` (`self.CurLocation`) (`self.TargetLocation_0`) _newtrack_0_2)))
        (:`Finished`
          (`self.OnSpwanEvent`)
          (if (`KismetStringLibrary.IsEmpty` (`self.EndAnimation Name`))
            (`self.ReturnPool`)
            (else
              (bind _returnvalue_5 (`SpineSkeletonAnimationComponent.SetAnimation` (`self.AnimComp`) 0 (`self.EndAnimation Name`) false))
              (bind _output_get (set `self.NewVar_0` _returnvalue_5))
              (add `TrackEntry.AnimationComplete` _output_get (delegate `CustomEvent_0`)))))))))

(event `CustomEvent_0`
  (params (entry :type "TrackEntry Object Reference"))
  (clear `TrackEntry.AnimationComplete` (`self.NewVar_0`))
  (`self.ReturnPool`))

(fn `UserConstructionScript`)