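; Blueprint template for a penetrating laser bullet that damages mice in its attack row, shown with a Spine animation.
; On init it plays the animation and immediately hits every mouse the row's line manager returns for an offset location and line type.
; Successful hits mark the mouse hurt and apply the bullet's buff.
; Though the animation is set to loop, its first completion event returns the bullet to the pool.
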(event `self.ReceiveBeginPlay`
  (`self.InitSpineShow`))

(event `self.OnInit`
  (bind _returnvalue (`self.SetAnimation` 0 "Def"))
  (bind _output_get (set `self.NewVar_0` _returnvalue))
  (add `TrackEntry.AnimationComplete` _output_get (delegate `CustomEvent_0`))
  (bind _returnvalue_2 (`GameMapInstance.GetMouseManagerComponent_Static`))
  (bind _returnvalue_3 (`MouseManagerComponent.GetMouseLineManager` _returnvalue_2 (`self.AttackRow`)))
  (`/Engine/EditorBlueprintResources/StandardMacros.IsValid` _returnvalue_3
    (:`Is Valid`
      (for _array_element (`MouseLineManager.GetMouseByLocation` _returnvalue_3 (- (`self.K2_GetActorLocation`) (0.0 50.0 0.0)) (`self.Mouse Line Type`))
        (`/Engine/EditorBlueprintResources/StandardMacros.IsValid` _array_element
          (:`Is Valid`
            (bind _returnvalue_4 (`self.GetCurATK`))
            (bind _returnvalue_5 (`MouseActor.BeHit` _array_element self _returnvalue_4 "Panetrate"))
            (if _returnvalue_5
              (`MouseActor.SetbIsHurt` _array_element true)
              (`MouseActor.ParseBuff_Information` _array_element (`self.M_FItem_Buff`) self))))))))

(event `CustomEvent_0`
  (params (entry :type "TrackEntry Object Reference"))
  (clear `TrackEntry.AnimationComplete` (`self.NewVar_0`))
  (`self.ReturnPool`))

(fn `OnReset`)

(fn `UserConstructionScript`)