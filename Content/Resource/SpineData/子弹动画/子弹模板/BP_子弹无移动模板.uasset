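; Template Blueprint for stationary bullets rendered with Spine animation, pooled for reuse.
; BeginPlay initializes the Spine display; OnInit starts the looping "Def" animation and listens for its first completion.
; That completion fires the spawn event, then either returns the bullet to the pool or, if an end animation is named, plays it once before pooling.
; Each completion handler unbinds itself, so the looping animation triggers only once.
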(event `self.ReceiveBeginPlay`
  (`self.InitSpineShow`))

(event `self.OnInit`
  (bind _returnvalue (`SpineSkeletonAnimationComponent.SetAnimation` (`self.AnimComp`) 0 "Def" true))
  (bind _output_get (set `self.NewVar_0` _returnvalue))
  (add `TrackEntry.AnimationComplete` _output_get (delegate `CustomEvent_0`)))

(event `CustomEvent_0`
  (params (entry :type "TrackEntry Object Reference"))
  (clear `TrackEntry.AnimationComplete` (`self.NewVar_0`))
  (if (`KismetStringLibrary.IsEmpty` (`self.EndAnimation Name`))
    (`self.OnSpwanEvent`)
    (`self.ReturnPool`)
    (else
      (bind _returnvalue (`SpineSkeletonAnimationComponent.SetAnimation` (`self.AnimComp`) 0 (`self.EndAnimation Name`) false))
      (bind _output_get (set `self.NewVar_1` _returnvalue))
      (add `TrackEntry.AnimationComplete` _output_get (delegate `CustomEvent_1`))
      (`self.OnSpwanEvent`))))

(event `CustomEvent_1`
  (params (entry :type "TrackEntry Object Reference"))
  (clear `TrackEntry.AnimationComplete` (`self.NewVar_1`))
  (`self.ReturnPool`))

(fn `UserConstructionScript`)