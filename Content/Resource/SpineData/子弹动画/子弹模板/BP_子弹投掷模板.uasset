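; Template Blueprint for a pooled, thrown (lobbed) projectile with a Spine visual.
; On init, a timeline feeds flight time and height values into ShootCruve, which yields the position along an arc toward the target, capped by MaxHight.
; Collision is disabled on pool init and switched to query-only at landing, with Hit called directly if no first hit result is found.
; OnHit stops the timeline.
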(event `self.ReceiveBeginPlay`
  (`self.InitSpineShow`))

(event `self.OnPoolInit`
  (`PrimitiveComponent.SetCollisionEnabled` (`self.M_SphereCollision`) "NoCollision"))

(event `self.OnInit`
  (`ShootCruveComponent.InitTarget` (`self.ShootCruve`))
  (bind _returnvalue (`FVMGameInstance.GetGameConfig_GameEFEnabled`))
  (if _returnvalue
    _
    (else
      _))
  (set `ShootCruveComponent.MaxHight` (`self.Max Hight`) (`self.ShootCruve`))
  (bind (_direction _flytime _flymaxhight) (`Timeline|Timeline_0` :!via `PlayFromStart` :!label _label)
    (:`Update`
      (bind _returnvalue_2 (`ShootCruveComponent.GetCurveLine` (`self.ShootCruve`) _flytime _flymaxhight))
      (`self.K2_SetActorLocation` _returnvalue_2))
    (:`Finished`
      (`PrimitiveComponent.SetCollisionEnabled` (`self.M_SphereCollision`) "QueryOnly")
      (if (not (`self.GetFirstHitResult`))
        (`self.Hit`)))))

(event `self.OnHit`
  (params (AttackType :type "EFlyItemAttackType Enum" :default "Def"))
  (goto _label :!via `Stop`))

(fn `UserConstructionScript`)