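; Slow-down buff for projectiles of Ice-category cards, with a default Rate of one half set on init.
; When initialized with its source object, it traces the flying item back to the card that fired it and checks that card's category.
; If both the card and the GamePlayer, fetched from the card manager's dynamic properties, are Ice, it multiplies Rate by the player's "other rate" bonus.
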(event `self.OnInit`
  (`parent.OnInit`)
  (set `self.Rate` 0.5))

(event `self.OnDefObjectInit`
  (params (Value :type "Object Object Reference"))
  (bind _asfly_item_actor (cast `FlyItemActor` Value))
  (bind _ascard_actor (cast `CardActor` (`FlyItemActor.GetFlyParentActor` _asfly_item_actor)))
  (bind _returnvalue (`CardActor.GetCardData` _ascard_actor))
  (if (`|EnumEquality` (`.GamePropertyCategory` (break `ItemCard` _returnvalue)) "Ice")
    (bind _returnvalue_2 (`GameMapInstance.GetGameMapInstance`))
    (bind _returnvalue_3 (`GameMapInstance.GetCardManagerComponent_Static` _returnvalue_2))
    (bind (_value _returnvalue_4) (`self.GetObjectProperty` (`CardManagerComponent.GetDynamicProperty` _returnvalue_3) "GamePlayer"))
    (if _returnvalue_4
      (bind _asgame_player (cast `GamePlayer` _value))
      (if (`|EnumEquality` (`.GamePropertyCategory` (break `ItemHeroBase` (`GamePlayer.GetPlayerData` _asgame_player))) "Ice")
        (set `self.Rate` (* (`self.Rate`) (`GamePlayer.GetPlayerOtherRate` _asgame_player)))))))