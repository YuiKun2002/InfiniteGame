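; BP_WaterUp is a Spine-animated upper water effect that plays a looping "shang" animation with a raised time scale.
; On BeginPlay it spawns a companion BP_WaterDown, whose SpineBoneFollower tracks this actor's "bone" by position only.
; Events move the actor and hide or show the companion on end and init.
; SetRenderLayer sorts this effect just below the given layer and passes the layer above to the companion.
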(event `self.ReceiveBeginPlay`
  (`self.InitSpineShow`)
  (`self.SetAnimation` 0 "shang")
  (bind _returnvalue (`|SpawnActorFromClass` "/Game/Resource/SpineData/水动画/BP_WaterDown.BP_WaterDown_C" (`KismetMathLibrary.MakeTransform` (0.0 0.0 0.0)) "Undefined" "OverrideRootScale" null null))
  (set `self.NewVar_0` _returnvalue)
  (bind _spinebonefollower (`/Game/Resource/SpineData/水动画/BP_WaterDown.SpineBoneFollower` _returnvalue))
  (set `SpineBoneFollowerComponent.Target` self _spinebonefollower)
  (set `SpineBoneFollowerComponent.BoneName` "bone" _spinebonefollower)
  (set `SpineBoneFollowerComponent.UseRotation` false _spinebonefollower)
  (set `SpineBoneFollowerComponent.UseScale` false _spinebonefollower)
  (set `SpineBoneFollowerComponent.UseComponentTransform` false _spinebonefollower)
  (set `SpineBoneFollowerComponent.UsePosition` true _spinebonefollower))

(event `self.OnMove`
  (params (Location :type "Vector Structure (by ref)"))
  (`self.K2_SetActorLocation` Location))

(event `self.OnSetRenderLayer`
  (params (Layer :type "Integer (by ref)"))
  (`self.SetRenderLayer` Layer))

(event `self.OnEnd`
  (`self.SetActorHiddenInGame` (`self.NewVar_0`) true))

(event `self.OnInit`
  (`self.SetActorHiddenInGame` (`self.NewVar_0`) false))

(fn `SetRenderLayer`
  (params (Layer :type Integer))
  (bind _output_get (set `self.Layer` Layer))
  (`PrimitiveComponent.SetTranslucentSortPriority` (`self.AnimRenderComp`) (- _output_get 1))
  (`/Game/Resource/SpineData/水动画/BP_WaterDown.SetRenderLayer` (`self.NewVar_0`) (+ _output_get 1)))

(fn `UserConstructionScript`
  (`self.SetAnimationTimeScale` 0 10.0))