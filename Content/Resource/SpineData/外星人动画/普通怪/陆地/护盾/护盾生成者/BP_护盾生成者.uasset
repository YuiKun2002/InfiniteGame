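; Shield generator Blueprint for a normal land alien enemy, handling projectile hits on its shield component.
; When a FlyItemActor with attack card type ENone overlaps ShieldComp, its current ATK and attack type are passed to BeHit.
; If BeHit succeeds, the hurt flag is set and the projectile's Hit is called.
; The construction script only runs the parent's.
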(event `self.ShieldComp.OnComponentBeginOverlap`
  (params (OverlappedComponent :type "PrimitiveComponent Object Reference") (OtherActor :type "Actor Object Reference") (OtherComp :type "PrimitiveComponent Object Reference") (OtherBodyIndex :type Integer) (bFromSweep :type Boolean) (SweepResult :type "HitResult Structure (by ref)"))
  (bind _asfly_item_actor (cast `FlyItemActor` OtherActor))
  (if (`|EnumEquality` (`FlyItemActor.M_AttackCardType` _asfly_item_actor) "E_None")
    (bind _returnvalue (`FlyItemActor.GetCurATK` _asfly_item_actor))
    (bind _m_flycondition_m_flyitemattacktype (break `lyItem_PropertyCondition` (`FlyItemActor.M_FlyCondition` _asfly_item_actor)))
    (bind _returnvalue_2 (`self.BeHit` _asfly_item_actor _returnvalue _m_flycondition_m_flyitemattacktype))
    (if _returnvalue_2
      (`self.SetbIsHurt` true)
      (`FlyItemActor.Hit` _asfly_item_actor))))

(fn `UserConstructionScript`
  (`parent.UserConstructionScript`))