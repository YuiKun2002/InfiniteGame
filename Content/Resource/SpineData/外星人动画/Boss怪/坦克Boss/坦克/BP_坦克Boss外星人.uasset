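; Tank boss alien that attacks the card grid with a laser and missiles, and spawns an explosion on death.
; The laser spawns a visual actor, then clears cards along its GetMouseLine row and the row above, prioritizing card ID 1 per cell and registering each loss via ResourceAddBadCard.
; Missiles launch from left and right mounts toward random map cells.
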(event `self.OnSpawnLaser`
  (bind (_returnvalue_x _returnvalue_y _returnvalue_z) (`KismetMathLibrary.BreakVector` (`self.K2_GetActorLocation`)))
  (bind (_relativelocation_x _relativelocation_y _relativelocation_z) (`KismetMathLibrary.BreakVector` (`SceneComponent.RelativeLocation` (`self.Scene_M_Laser`))))
  (bind _returnvalue (`|SpawnActorFromClass` "/Game/Resource/SpineData/外星人动画/Boss怪/坦克Boss/坦克/BP_坦克激光.BP_坦克激光_C" (`KismetMathLibrary.MakeTransform` (+ (`KismetMathLibrary.MakeVector` _relativelocation_y _relativelocation_x _relativelocation_z) (`KismetMathLibrary.MakeVector` _returnvalue_x _returnvalue_y _returnvalue_z))) "Undefined" "OverrideRootScale" null null))
  (`self.InitSpineShow` _returnvalue)
  (`self.SetSpineRenderLayer` _returnvalue 9999)
  (`self.SetRotation` _returnvalue -90.0)
  (bind _returnvalue_2 (`self.GetMouseLine`))
  (`self.SpawnLine` (break `Line` _returnvalue_2) (`.Col` (break `Line` _returnvalue_2)))
  (if (not (== (break `Line` _returnvalue_2) 0))
    (`self.SpawnLine` (- (break `Line` _returnvalue_2) 1) (`.Col` (break `Line` _returnvalue_2)))))

(event `self.OnSpawnMissile`
  (bind (_returnvalue_x _returnvalue_y _returnvalue_z) (`KismetMathLibrary.BreakVector` (`self.K2_GetActorLocation`)))
  (bind (_returnvalue_x_2 _returnvalue_y_2 _returnvalue_z_2) (`KismetMathLibrary.BreakVector` (`self.K2_GetActorLocation`)))
  (bind (_relativelocation_x _relativelocation_y _relativelocation_z) (`KismetMathLibrary.BreakVector` (`SceneComponent.RelativeLocation` (`self.Scene_M_Left`))))
  (bind (_relativelocation_x_2 _relativelocation_y_2 _relativelocation_z_2) (`KismetMathLibrary.BreakVector` (`SceneComponent.RelativeLocation` (`self.Scene_M_Right`))))
  (`self.SpawnMissileLocation` (+ (`KismetMathLibrary.MakeVector` _relativelocation_y_2 _relativelocation_x_2 _relativelocation_z_2) (`KismetMathLibrary.MakeVector` _returnvalue_x _returnvalue_y _returnvalue_z)))
  (`self.SpawnMissileLocation` (+ (`KismetMathLibrary.MakeVector` _relativelocation_y _relativelocation_x _relativelocation_z) (`KismetMathLibrary.MakeVector` _returnvalue_x_2 _returnvalue_y_2 _returnvalue_z_2))))

(event `self.OnDead`
  (bind _returnvalue (`|SpawnActorFromClass` "/Game/Resource/SpineData/外星人动画/Boss怪/坦克Boss/坦克/BP_爆炸动画.BP_爆炸动画_C" (`KismetMathLibrary.MakeTransform` (`self.K2_GetActorLocation`)) "Undefined" "OverrideRootScale" null null))
  (`MagicMasterHpAddtionBuff.Init` _returnvalue self))

(fn `SpawnLine`
  (params (Row :type Integer) (Col :type Integer))
  (locals (NewLocalVar_0 :type Integer :default 0) (NewLocalVar_1 :type "Float (single-precision)" :default 0.0) (NewLocalVar_3 :type "Array of EObjectTypeQuery Enum") (NewLocalVar_2 :type Integer))
  (bind _output_get (set `local.NewLocalVar_2` Col))
  (if (== _output_get -1)
    (bind _returnvalue (`GameMapInstance.GetGameMapInstance`))
    (bind _returnvalue_2 (`MesheControllComponent.GetMapMeshRowAndCol` (`GameMapInstance.M_MesheControllComponent` _returnvalue)))
    (set `local.NewLocalVar_2` (- (`.Col` (break `Line` _returnvalue_2)) 1)))
  (bind _returnvalue_3 (`GameMapInstance.GetGameMapInstance`))
  (for _index (range (+ (`local.NewLocalVar_2`) 1))
    (bind _returnvalue_4 (`MesheControllComponent.GetMapMesh` (`GameMapInstance.M_MesheControllComponent` _returnvalue_3) Row _index))
    (bind _returnvalue_5 (`MapMeshe.GetUIMapMeshe` _returnvalue_4))
    (`/Engine/EditorBlueprintResources/StandardMacros.IsValid` _returnvalue_5
      (:`Is Valid`
        (bind _returnvalue_6 (`UI_MapMeshe.EradicateCardByID` _returnvalue_5 1))
        (if _returnvalue_6
          (`ResourceManagerComponent.ResourceAddBadCard`)
          (else
            (bind _returnvalue_7 (`UI_MapMeshe.EradicateCard` _returnvalue_5))
            (if _returnvalue_7
              (`ResourceManagerComponent.ResourceAddBadCard`))))))))

(fn `SpawnMissileLocation`
  (params (NewLocation :type "Vector Structure"))
  (bind _returnvalue (`|SpawnActorFromClass` "/Game/Resource/SpineData/外星人动画/Boss怪/坦克Boss/坦克/BP_坦克导弹.BP_坦克导弹_C" (`KismetMathLibrary.MakeTransform` (0.0 0.0 0.0)) "DontSpawnIfColliding" "OverrideRootScale" null null))
  (`self.K2_SetActorLocation` _returnvalue NewLocation false false)
  (`self.SetSpineRenderLayer` _returnvalue 9999)
  (bind _returnvalue_2 (`GameMapInstance.GetGameMapInstance`))
  (bind _m_meshecontrollcomponent (`GameMapInstance.M_MesheControllComponent` _returnvalue_2))
  (bind _returnvalue_3 (`MesheControllComponent.GetMapMeshRowAndCol` _m_meshecontrollcomponent))
  (bind _returnvalue_4 (`MesheControllComponent.GetMapMeshLocation` _m_meshecontrollcomponent (`KismetMathLibrary.RandomInteger` (break `Line` _returnvalue_3)) (`KismetMathLibrary.RandomInteger` (- (`.Col` (break `Line` _returnvalue_3)) 1))))
  (`DaLiShenMissile.SetTarget` _returnvalue _returnvalue_4))

(fn `UserConstructionScript`
  (`parent.UserConstructionScript`))