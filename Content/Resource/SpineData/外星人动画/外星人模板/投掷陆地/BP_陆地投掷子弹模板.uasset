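; Template Blueprint for a Spine-animated land-thrown projectile that damages cards on landing.
; Init stores the target, then a timeline moves the actor along an arc to it.
; On arrival it damages living cards in a list until one dies, or falls back to a debug-drawn sphere trace if none was hit.
; Killed cards are recorded as bad cards, and the projectile destroys itself after its Fracture animation.
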(event `self.ReceiveBeginPlay`
  (`self.InitSpineShow`)
  (`self.SetAnimation` 0 "Def"))

(event `self.Init`
  (params (TargetLocation :type "Vector Structure (by ref)") (CurLocation :type "Vector Structure (by ref)") (TargetHitCard :type "Array of CardActor Object Reference (by ref)"))
  (bind _returnvalue (`self.K2_GetActorLocation`))
  ;[1 1 1] 初始化条件以及位置信息
  (set `self.Target Location` TargetLocation)
  (set `self.Target Hit Card` TargetHitCard)
  (set `self.CurLocation` CurLocation)
  (set `self.bHit` false)
  ;[1 1 1] 从起始点飞向目标点的抛物线
  (bind (_direction _locationtime _highttime) (`Timeline|FlyTarget` :!via `PlayFromStart`)
    (:`Update`
      (bind _outlocation (`GameSystemFunction.GetCurveLineByTimeLineBlue` (`self.CurLocation`) (`self.Target Location`) 80.0 _locationtime _highttime))
      (`self.K2_SetActorLocation` _outlocation))
    (:`Finished`
      ;[1 1 1] 如果当前网格存在的卡片有效，则直接消耗血量，死亡则记录卡片损坏
      (for _array_element _
        (`/Engine/EditorBlueprintResources/StandardMacros.IsValid` _array_element
          (:`Is Valid`
            (bind _returnvalue_2 (`CardActor.GetCurrentHP` _array_element))
            (if (> _returnvalue_2 0.0)
              (set `self.bHit` true)
              (bind _returnvalue_3 (`CardActor.UpdateCardState` _array_element (`self.ATK Value`) (`self.Up HP Value`)))
              (if _returnvalue_3
                (`CardActor.KillCard` _array_element)
                (`ResourceManagerComponent.ResourceAddBadCard`)
                (break))))))
      (if (`self.bHit`)
        (bind _returnvalue_4 (`self.AddAnimation` 0 "Fracture" false 0.1))
        (add `TrackEntry.AnimationComplete` _returnvalue_4 (delegate `AnimComplete`))
        (else
          ;[1 1 1] 之前的卡片全部都失效了，则临时创建球体范围检测，检测当前网格存在的卡片，并且消耗当前卡片的血量
          (bind _returnvalue_5 (`self.AddAnimation` 0 "Fracture" false 0.1))
          (add `TrackEntry.AnimationComplete` _returnvalue_5 (delegate `AnimComplete`))
          (bind _outhit (`KismetSystemLibrary.SphereTraceSingle` :`Start` _returnvalue :`End` _returnvalue :`Radius` 20.0 :`TraceChannel` "TraceTypeQuery3" :`DrawDebugType` "ForDuration"))
          (bind _ascard_actor (cast `CardActor` (`.HitActor` (`GameplayStatics.BreakHitResult` _outhit))))
          (bind _returnvalue_6 (`CardActor.GetCurrentHP` _ascard_actor))
          (if (> _returnvalue_6 0.0)
            (bind _returnvalue_7 (`CardActor.UpdateCardState` _ascard_actor (`self.ATK Value`) (`self.Up HP Value`)))
            (if _returnvalue_7
              (`CardActor.KillCard` _ascard_actor)
              (`ResourceManagerComponent.ResourceAddBadCard`))))))))

(event `AnimComplete`
  (params (entry :type "TrackEntry Object Reference"))
  (`self.K2_DestroyActor`))

(fn `UserConstructionScript`)