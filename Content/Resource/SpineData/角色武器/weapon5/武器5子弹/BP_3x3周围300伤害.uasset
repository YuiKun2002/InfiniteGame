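; Area damage effect for weapon 5's bullets that hits mouse enemies in the surrounding 3x3 area.
; On init it sets its attack and runs a stationary multi-sphere trace at its own location.
; Each MouseActor hit receives a Burn buff and a Bomb-type hit, and is flagged hurt if that hit succeeds.
; The trace's debug drawing and a location print are still enabled, and the first non-mouse hit stops processing.
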(event `self.OnInit`
  (bind _returnvalue (`self.K2_GetActorLocation`))
  (`self.SetCurATK` 300.0)
  (`KismetSystemLibrary.PrintString` (`KismetStringLibrary.Conv_VectorToString` _returnvalue))
  (bind _outhits (`KismetSystemLibrary.SphereTraceMulti` :`Start` _returnvalue :`End` _returnvalue :`Radius` 90.0 :`TraceChannel` "TraceTypeQuery4" :`DrawDebugType` "ForDuration"))
  (for _array_element _outhits
    (bind _asmouse_actor (cast `MouseActor` (`.HitActor` (`GameplayStatics.BreakHitResult` _array_element))))
    (`MouseActor.ParseBuff_Information` _asmouse_actor (make `GameBuffInfor` (`|MakeMap` "Burn" 0.2 :!type "EGameBuffTag Enum" :!valuetype "Float (single-precision)") (`|MakeMap` "Burn" "/Game/Resource/BP/Data/Buff/BP_灼烧Buff.BP_灼烧Buff_C" :!type "EGameBuffTag Enum" :!valuetype "BuffDynamicProperty Class Reference")) self)
    (bind _returnvalue_2 (`MouseActor.BeHit` _asmouse_actor self 300.0 "Bomb"))
    (if _returnvalue_2
      (`MouseActor.SetbIsHurt` _asmouse_actor true))))

(fn `UserConstructionScript`)