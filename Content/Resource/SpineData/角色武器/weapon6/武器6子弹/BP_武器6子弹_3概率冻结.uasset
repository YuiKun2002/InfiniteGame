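; Weapon 6 bullet variant that has a small random chance to freeze and otherwise slows.
; On each reset it runs the parent logic, then, if its fly parent is a valid GamePlayer, takes that player's line row as its attack row.
; It then rolls once to set its buff to either a short Freeze or a longer SlowDown that uses the weapon 6 slow buff property.
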(fn `OnReset`
  (`parent.OnReset`)
  (bind _asgame_player (cast `GamePlayer` (`self.GetFlyParentActor`)))
  (`/Engine/EditorBlueprintResources/StandardMacros.IsValid` _asgame_player
    (:`Is Valid`
      (bind _returnvalue_row (break `Line` (`GamePlayer.GetLine` _asgame_player)))
      (set `self.AttackRow` _returnvalue_row)
      (if (<= (`KismetMathLibrary.RandomIntegerInRange` 0 100) 3)
        (`self.ResetBuff` (`|MakeMap` "Freeze" 2.0 :!type "EGameBuffTag Enum" :!valuetype "Float (single-precision)") (`|MakeMap` "Freeze" :!type "EGameBuffTag Enum" :!valuetype "BuffDynamicProperty Class Reference"))
        (else
          (`self.ResetBuff` (`|MakeMap` "SlowDown" 5.0 :!type "EGameBuffTag Enum" :!valuetype "Float (single-precision)") (`|MakeMap` "SlowDown" "/Game/Resource/SpineData/角色武器/weapon6/Skill/BP_减速Buff_60p_武器6.BP_减速Buff_60p_武器6_C" :!type "EGameBuffTag Enum" :!valuetype "BuffDynamicProperty Class Reference")))))))

(fn `UserConstructionScript`)