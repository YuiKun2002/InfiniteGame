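; Lava-tile flame actor with a looping Spine animation that gives an Accelerate buff to mouse units on its row.
; A looping timer, cleared on destruction, runs a small sphere trace for a MouseActor and compares line rows before applying the buff.
; The same tick hides the flame unless its card count is non-zero or the previous trace found a matching mouse.
; The trace still has one-frame debug drawing enabled.
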(event `self.ReceiveDestroyed`
  (`KismetSystemLibrary.K2_ClearAndInvalidateTimerHandle` (`self.TimerHd`)))

(event `self.ReceiveBeginPlay`
  (bind _returnvalue (`KismetSystemLibrary.K2_SetTimerDelegate` (delegate `CustomEvent_0`) 0.2 true))
  (set `self.TimerHd` _returnvalue))

(event `CustomEvent_0`
  (bind _returnvalue (- (`self.K2_GetActorLocation`) (0.0 0.0 7.0)))
  (bind _returnvalue_2 (`self.GetCardNums`))
  (if (== _returnvalue_2 0)
    (if (`self.bMouse`)
      (`self.SetActorHiddenInGame` false)
      (else
        (`self.SetActorHiddenInGame` true)))
    (else
      (`self.SetActorHiddenInGame` false)))
  (bind _outhit (`KismetSystemLibrary.SphereTraceSingle` :`Start` _returnvalue :`End` _returnvalue :`Radius` 27.0 :`TraceChannel` "TraceTypeQuery11" :`DrawDebugType` "ForOneFrame"))
  (bind _asmouse_actor (cast `MouseActor` (`.HitActor` (`GameplayStatics.BreakHitResult` _outhit)))
    (:`then`
      (bind _returnvalue_3 (`MouseActor.GetMouseLine` _asmouse_actor))
      (bind _returnvalue_4 (`self.GetLine`))
      (if (== (`.Row` (break `Line` _returnvalue_4)) (`.Row` (break `Line` _returnvalue_3)))
        (set `self.bMouse` true)
        (`MouseActor.ParseBuff_Information` _asmouse_actor (make `GameBuffInfor` (`|MakeMap` "Accelerate" 0.2 :!type "EGameBuffTag Enum" :!valuetype "Float (single-precision)") (`|MakeMap` "Accelerate" :!type "EGameBuffTag Enum" :!valuetype "BuffDynamicProperty Class Reference")) self)
        (else
          (set `self.bMouse` false))))
    (:`CastFailed`
      (set `self.bMouse` false))))

(fn `UserConstructionScript`
  (`self.SetAnimation` 0 "animation"))