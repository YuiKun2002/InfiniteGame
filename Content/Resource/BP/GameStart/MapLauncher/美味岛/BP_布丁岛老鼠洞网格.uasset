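; Mouse hole grid cell for the Pudding Island map that periodically spawns mice onto its lane.
; On init it looks up the map mesh at its row and column and kills all cards on that cell.
; A bound tick callback accumulates delta time and, about every 60 seconds, spawns a randomly picked mouse from its name list, slightly below the hole's location.
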(event `CustomEvent_0`
  (bind _returnvalue (`GameMapInstance.GetGameMapInstance`))
  (bind _returnvalue_2 (`self.GetMouseLine`))
  (bind _returnvalue_3 (`MesheControllComponent.GetMapMesh` (`GameMapInstance.M_MesheControllComponent` _returnvalue) (break `Line` _returnvalue_2) (`.Col` (break `Line` _returnvalue_2))))
  (bind _returnvalue_4 (`MapMeshe.GetUIMapMeshe` _returnvalue_3))
  (`UI_MapMeshe.KillAllCards` _returnvalue_4))

(event `self.ReceiveBeginPlay`
  (`parent.ReceiveBeginPlay`)
  (add `self.OnInit` (delegate `CustomEvent_0`))
  (add `self.Tick` (delegate `TickUpdate`)))

(event `TickUpdate` :!signature `self.Tick`
  (params (DeltaTime :type "Float (double-precision)"))
  (if (>= (`self.Delta Time`) 60.0)
    (set `self.Delta Time` 0.0)
    (bind _returnvalue (`self.GetMouseLine`))
    (bind _name (`self.GetMouseName`))
    (`MouseSpawnManager.MakeNewMouseByName` "/Game/Resource/BP/Data/MouseData/MouseData.MouseData" _name (make `Line` (break `Line` _returnvalue) (`.Col` (break `Line` _returnvalue))) (+ (`self.K2_GetActorLocation`) (0.0 0.0 -15.0)))
    (else
      (set `self.Delta Time` (+ DeltaTime (`self.Delta Time`))))))

(fn `GetMouseName`
  (returns (Name :type String))
  (return (`KismetArrayLibrary.Array_Random` (`self.List`))))

(fn `UserConstructionScript`
  (`parent.UserConstructionScript`))