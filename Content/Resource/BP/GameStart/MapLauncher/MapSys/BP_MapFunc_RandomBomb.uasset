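; Map function that periodically drops a random bomb on one of the mice in the level until the game ends.
; A self-rebinding cycle through the RandomTimeBombEve dispatcher sets a one-shot timer of random length, roughly 7–13 seconds.
; Each firing spawns BP_MapFunc_RandomBombAnim at a random mouse's location, skipped if colliding, then re-arms the timer.
; Game over or destruction unbinds the dispatcher and clears the timer.
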(event `self.OnFuncInitEvent`
  (add `self.RandomTimeBombEve` (delegate `LoopEvent`))
  (`self.RandomTimeBombEve`))

(event `LoopEvent`
  (bind _returnvalue (`KismetSystemLibrary.K2_SetTimerDelegate` (delegate `LoopBody`) (`KismetMathLibrary.RandomFloatInRange` 7.0 13.0)))
  (set `self.TimeHand` _returnvalue))

(event `LoopBody`
  (`KismetSystemLibrary.K2_ClearAndInvalidateTimerHandle` (`self.TimeHand`))
  (if (`self.GetGameOver`)
    ;[1 1 1] 游戏结束
    (clear `self.RandomTimeBombEve`)
    (`KismetSystemLibrary.K2_ClearAndInvalidateTimerHandle` (`self.TimeHand`))
    (else
      (bind _outallmouse (`MouseManagerComponent.GetAllMouse`))
      (if (> (`KismetArrayLibrary.Array_Length` _outallmouse) 0)
        (bind _outitem (`KismetArrayLibrary.Array_Random` _outallmouse))
        (`/Engine/EditorBlueprintResources/StandardMacros.IsValid` _outitem
          (:`Is Valid`
            (`|SpawnActorFromClass` "/Game/Resource/BP/GameStart/MapLauncher/MapSys/BP_MapFunc_RandomBombAnim.BP_MapFunc_RandomBombAnim_C" (`KismetMathLibrary.MakeTransform` (`self.K2_GetActorLocation` _outitem)) "DontSpawnIfColliding" "OverrideRootScale" null null)
            (`self.RandomTimeBombEve`))
          (:`Is Not Valid`
            (`self.RandomTimeBombEve`)))
        (else
          (`self.RandomTimeBombEve`))))))

(event `self.ReceiveDestroyed`
  (clear `self.RandomTimeBombEve`)
  (`KismetSystemLibrary.K2_ClearAndInvalidateTimerHandle` (`self.TimeHand`)))

(fn `UserConstructionScript`)