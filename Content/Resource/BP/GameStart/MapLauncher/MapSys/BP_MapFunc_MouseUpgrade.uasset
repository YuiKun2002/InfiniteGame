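; BP_MapFunc_MouseUpgrade is a map function that periodically strengthens every mouse enemy in the level.
; On init it starts a looping four-second timer that, until game over, gives each valid mouse a timed Accelerate buff and partial damage reduction, then shows an on-screen announcement.
; The timer is cleared once the game ends or when the actor is destroyed.
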(event `self.OnFuncInitEvent`
  (bind _returnvalue (`KismetSystemLibrary.K2_SetTimerDelegate` (delegate `CustomEvent_0`) 4.0 true))
  (set `self.NewVar_0` _returnvalue))

(event `self.ReceiveDestroyed`
  (`KismetSystemLibrary.K2_ClearAndInvalidateTimerHandle` (`self.NewVar_0`) :!label _label))

(event `CustomEvent_0`
  (if (`self.GetGameOver`)
    (goto _label)
    (else
      (bind _outallmouse (`MouseManagerComponent.GetAllMouse`))
      (for _array_element _outallmouse
        (`/Engine/EditorBlueprintResources/StandardMacros.IsValid` _array_element
          (:`Is Valid`
            (`MouseActor.ParseBuff_Information` _array_element (make `GameBuffInfor` (`|MakeMap` "Accelerate" 5.0 :!type "EGameBuffTag Enum" :!valuetype "Float (single-precision)") (`|MakeMap` "Accelerate" :!type "EGameBuffTag Enum" :!valuetype "BuffDynamicProperty Class Reference")) self)
            (`MouseActor.SetIgnoreHurtValue` _array_element 0.4))))
      (bind _returnvalue (`GameMapInstance.GetVSManagerComponent_Static`))
      (`/Engine/EditorBlueprintResources/StandardMacros.IsValid` _returnvalue
        (:`Is Valid`
          (`VSManagerComponent.ShowText` _returnvalue "老鼠大军被强化！获得35%加速和40%伤害减免"))))))

(fn `UserConstructionScript`
  (`parent.UserConstructionScript`))