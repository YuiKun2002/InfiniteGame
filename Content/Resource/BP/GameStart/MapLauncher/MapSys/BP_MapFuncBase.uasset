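; BP_MapFuncBase is a base Blueprint for map function objects in the MapLauncher's map system.
; On BeginPlay it binds an empty init event to OnFuncInit, which subclasses implement with their own setup.
; It stores a Parent reference through getter and setter functions.
; GetGameOver forwards the game map instance's game-over state and returns true when that instance is invalid.
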(event `self.ReceiveBeginPlay`
  ;[1 1 1] 初始绑定事件，事件由子类实现
  (add `self.OnFuncInit` (delegate `OnFuncInitEvent`)))

(event `OnFuncInitEvent`
  ;[1 1 1] 初始绑定事件，事件由子类实现
)

(fn `GetGameOver`
  (returns (GameOver :type Boolean))
  (bind _returnvalue (`GameMapInstance.GetGameMapInstance`))
  (`/Engine/EditorBlueprintResources/StandardMacros.IsValid` _returnvalue
    (:`Is Valid`
      (bind _returnvalue_2 (`GameMapInstance.GetGameOver` _returnvalue))
      (return _returnvalue_2))
    (:`Is Not Valid`
      (return true))))

(fn `GetParent`
  (returns (CurParent :type "/Game/Resource/BP/GameStart/MapLauncher/BP_MapLauncherBase Object Reference"))
  (return (`self.Parent`)))

(fn `SetParent`
  (params (NewParent :type "/Game/Resource/BP/GameStart/MapLauncher/BP_MapLauncherBase Object Reference"))
  (set `self.Parent` NewParent))

(fn `UserConstructionScript`)