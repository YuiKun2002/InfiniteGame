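; Random-bomb map effect actor that detonates once on spawn, damaging mice around it.
; On BeginPlay it initializes rotation, plays the bomb sound and runs a zero-length multi-sphere trace at its location.
; Each MouseActor hit is flagged hurt and takes Bomb damage equal to 85% of its total HP.
; Destroy-on-animation-end is set only when the trace reports a hit.
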(event `self.ReceiveBeginPlay`
  (bind _returnvalue (`self.K2_GetActorLocation`))
  (`self.InitRotation`)
  (`FVMGameInstance.PlayBGM_S_Static` "Bomb" "ItemAudio")
  (bind (_outhits _returnvalue_2) (`KismetSystemLibrary.SphereTraceMulti` _returnvalue _returnvalue 90.0 "TraceTypeQuery11"))
  (if _returnvalue_2
    (for _array_element _outhits
      (bind _asmouse_actor (cast `MouseActor` (`.HitActor` (`GameplayStatics.BreakHitResult` _array_element))))
      (bind _returnvalue_3 (`MouseActor.GetTotalHP` _asmouse_actor))
      (`MouseActor.SetbIsHurt` _asmouse_actor true)
      (`MouseActor.BeHit` _asmouse_actor self (* _returnvalue_3 0.85) "Bomb"))
    (`self.SetAnimationPlayEndDestroy`)))

(fn `UserConstructionScript`)