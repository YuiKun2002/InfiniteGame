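; Base map launcher Blueprint offering helpers that set up a level at game start.
; GenFunc loads soft-referenced BP_MapFuncBase classes, spawns and initializes them for bomb, mouse-upgrade and character features, and tracks them for cleanup on Destroyed.
; Card placement issues "/game play" text commands within grid bounds, while GenCards builds play-card structs from a DataTable.
; GenWater separately spawns a soft-loaded sprite actor at a default or supplied transform.
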(event `self.ReceiveDestroyed`
  (for _array_element (`self.Actors`)
    (`self.K2_DestroyActor` _array_element))
  (`KismetArrayLibrary.Array_Clear` (`self.Actors`)))

(fn `Gen_Water`
  (params (Trans :type "Transform Structure") (bUseDef :type Boolean :default true))
  (returns (WaterActor :type "SpriteActor Object Reference"))
  (locals (DefLocation :type "Transform Structure" :default "570.000000,100.000000,75.000000|0.000000,0.000000,-0.000000|0.980000,0.100000,1.500000") (softPath :type "SoftClassPath Structure" :default "/Game/Resource/Texture/Sprite/VS/Map/0/BP_MapWater.BP_MapWater_C"))
  (if (not bUseDef)
    (set `local.DefLocation` Trans))
  (bind _returnvalue (`KismetSystemLibrary.LoadClassAsset_Blocking` (`KismetSystemLibrary.Conv_SoftClassPathToSoftClassRef` (`local.softPath`))))
  (bind _assprite_actor (castclass `SpriteActor` _returnvalue))
  (bind _returnvalue_2 (`|SpawnActorFromClass` _assprite_actor (`local.DefLocation`) "DontSpawnIfColliding" "OverrideRootScale" null null))
  (return _returnvalue_2))

(fn `GenCards`
  (params (Cards :type "Map of String to Integer"))
  (returns (CardData :type "Map of String to /Game/Resource/BP/Data/CardData/DialogueChar/PlayCardStruct Structure"))
  (locals (CardsData :type "DataTable Soft Object Reference" :default "/Game/Resource/BP/Data/CardData/DialogueChar/DT_PlayCardsData.DT_PlayCardsData") (DataTableIns :type "DataTable Object Reference") (TargetData :type "Map of String to /Game/Resource/BP/Data/CardData/DialogueChar/PlayCardStruct Structure"))
  (`|ExecutionSequence`
    (:`then_0`
      ;[1 1 1] 初始化数据表
      (bind _returnvalue (`KismetSystemLibrary.LoadAsset_Blocking` (`local.CardsData`)))
      (bind _asdata_table (cast `DataTable` _returnvalue))
      (set `local.DataTableIns` _asdata_table))
    (:`then_1`
      ;[1 1 1] 生成对应数据
      (bind _keys (`BlueprintMapLibrary.Map_Keys` (`local.Cards`)))
      (for (_array_element _array_index) _keys
        (bind _values (`BlueprintMapLibrary.Map_Values` (`local.Cards`)))
        (bind _returnvalue_2 (`|GetDataTableRow` (`local.DataTableIns`) (`KismetStringLibrary.Conv_StringToName` _array_element))
          (:`then`
            (bind (_grade _id _playtype _playcategroy) (break `/Game/Resource/BP/Data/CardData/DialogueChar/PlayCardStruct` _returnvalue_2))
            (`BlueprintMapLibrary.Map_Add` (`local.TargetData`) _array_element (make `/Game/Resource/BP/Data/CardData/DialogueChar/PlayCardStruct` (`|GetArrayItem` _values _array_index) _id _playtype _playcategroy))))))
    (:`then_2`
      ;[1 1 1] 返回数据
      (return (`local.TargetData`)))))

(fn `GenCharForGame`
  (params (Cards :type "Map of String to /Game/Resource/BP/Data/CardData/DialogueChar/PlayCardStruct Structure"))
  (locals (NewLocalVar_2 :type "SoftClassPath Structure" :default "/Game/Resource/BP/GameStart/MapLauncher/MapSys/BP_MapFunc_Char.BP_MapFunc_Char_C"))
  (bind _newfunc (`self.GenFunc` (`local.NewLocalVar_2`)))
  (bind _asi_init_play_card_interface (cast `/Game/Resource/BP/Data/CardData/DialogueChar/I_InitPlayCardInterface` _newfunc))
  (`/Game/Resource/BP/Data/CardData/DialogueChar/I_InitPlayCardInterface.Init Card Data` _asi_init_play_card_interface (`local.Cards`)))

(fn `GenFunc`
  (params (FuncRes :type "SoftClassPath Structure"))
  (returns (NewFunc :type "/Game/Resource/BP/GameStart/MapLauncher/MapSys/BP_MapFuncBase Object Reference"))
  (bind _returnvalue (`KismetSystemLibrary.Conv_SoftClassPathToSoftClassRef` FuncRes))
  (if (`KismetSystemLibrary.IsValidSoftClassReference` _returnvalue)
    (bind _returnvalue_2 (`KismetSystemLibrary.LoadClassAsset_Blocking` _returnvalue))
    (bind _asbp_map_func_base (castclass `/Game/Resource/BP/GameStart/MapLauncher/MapSys/BP_MapFuncBase` _returnvalue_2))
    (bind _returnvalue_3 (`|SpawnActorFromClass` _asbp_map_func_base (`KismetMathLibrary.MakeTransform` (0.0 0.0 0.0)) "DontSpawnIfColliding" "OverrideRootScale" null null))
    (`/Game/Resource/BP/GameStart/MapLauncher/MapSys/BP_MapFuncBase.OnFuncInit` _returnvalue_3)
    (`KismetArrayLibrary.Array_Add` (`self.Actors`) _returnvalue_3)
    (return _returnvalue_3)))

(fn `MouseUpGrade`
  (locals (NewLocalVar_1 :type "SoftClassPath Structure" :default "/Game/Resource/BP/GameStart/MapLauncher/MapSys/BP_MapFunc_MouseUpgrade.BP_MapFunc_MouseUpgrade_C"))
  (`self.GenFunc` (`local.NewLocalVar_1`)))

(fn `PlayCardGroup`
  (params (PlayCol :type Integer) (PlayRows :type "Map of Integer to String"))
  (locals (Row :type Integer) (Col :type Integer))
  (bind _returnvalue (`GameMapInstance.GetGameMapInstance`))
  (`/Engine/EditorBlueprintResources/StandardMacros.IsValid` _returnvalue
    (:`Is Valid`
      (bind _m_meshecontrollcomponent (`GameMapInstance.M_MesheControllComponent` _returnvalue))
      (`/Engine/EditorBlueprintResources/StandardMacros.IsValid` _m_meshecontrollcomponent
        (:`Is Valid`
          (bind _returnvalue_2 (`MesheControllComponent.GetMapMeshRowAndCol` _m_meshecontrollcomponent))
          (set `local.Row` (break `Line` _returnvalue_2))
          (bind _output_get (set `local.Col` PlayCol))
          (if (not (>= _output_get (`.Col` (break `Line` _returnvalue_2))))
            (bind _keys (`BlueprintMapLibrary.Map_Keys` PlayRows))
            (for (_array_element _array_index) _keys
              (bind _values (`BlueprintMapLibrary.Map_Values` PlayRows))
              (if (< _array_element (`local.Row`))
                (`GameSystemFunction.AddGameinstructions` self (`KismetStringLibrary.Concat_StrStr` "/game play " (`|GetArrayItem` _values _array_index) " " (`KismetStringLibrary.Conv_IntToString` _array_element) "," (`KismetStringLibrary.Conv_IntToString` (`local.Col`))) false)))))))))

(fn `PlayCardGroups`
  (params (PlayCol :type Integer) (PlayRows :type "Array of String"))
  (locals (Row :type Integer) (Col :type Integer))
  (bind _returnvalue (`GameMapInstance.GetGameMapInstance`))
  (`/Engine/EditorBlueprintResources/StandardMacros.IsValid` _returnvalue
    (:`Is Valid`
      (bind _m_meshecontrollcomponent (`GameMapInstance.M_MesheControllComponent` _returnvalue))
      (`/Engine/EditorBlueprintResources/StandardMacros.IsValid` _m_meshecontrollcomponent
        (:`Is Valid`
          (bind _returnvalue_2 (`MesheControllComponent.GetMapMeshRowAndCol` _m_meshecontrollcomponent))
          (set `local.Row` (break `Line` _returnvalue_2))
          (bind _output_get (set `local.Col` PlayCol))
          (if (not (>= _output_get (`.Col` (break `Line` _returnvalue_2))))
            (for (_array_element _array_index) PlayRows
              (if (< _array_index (`local.Row`))
                (`GameSystemFunction.AddGameinstructions` self (`KismetStringLibrary.Concat_StrStr` "/game play " _array_element " " (`KismetStringLibrary.Conv_IntToString` _array_index) "," (`KismetStringLibrary.Conv_IntToString` (`local.Col`))) false)))))))))

(fn `RandomBomb`
  (locals (NewLocalVar_0 :type "SoftClassPath Structure" :default "/Game/Resource/BP/GameStart/MapLauncher/MapSys/BP_MapFunc_RandomBomb.BP_MapFunc_RandomBomb_C"))
  (`self.GenFunc` (`local.NewLocalVar_0`)))

(fn `UserConstructionScript`)