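; Obstacle actor of the mechanical bomb-throwing mouse that damages cards where it sits when its animation finishes.
; It initializes rotation on BeginPlay, then on animation end runs a zero-length capsule trace just above its location, with one-frame debug drawing.
; Each hit CardActor gets the attack values, and those reporting true are killed, followed by a ResourceAddBadCard call.
; The actor destroys itself after processing the hits.
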(event `self.ReceiveBeginPlay`
  (`self.InitRotation`))

(event `self.OnAnimationPlayEndBlueprint`
  (bind _returnvalue (+ (`self.K2_GetActorLocation`) (0.0 0.0 15.0)))
  (bind _outhits (`KismetSystemLibrary.CapsuleTraceMulti` :`Start` _returnvalue :`End` _returnvalue :`Radius` 25.0 :`TraceChannel` "TraceTypeQuery3" :`DrawDebugType` "ForOneFrame"))
  (for _array_element _outhits
    (bind _ascard_actor (cast `CardActor` (`.HitActor` (`GameplayStatics.BreakHitResult` _array_element))))
    (bind _returnvalue_2 (`CardActor.UpdateCardState` _ascard_actor (`self.ATK Value`) (`self.Up HP Value`)))
    (if _returnvalue_2
      (`CardActor.KillCard` _ascard_actor)
      (`ResourceManagerComponent.ResourceAddBadCard`)))
  (`self.K2_DestroyActor`))

(fn `UserConstructionScript`)