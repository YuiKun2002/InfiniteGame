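; Repair mouse's ladder (修理鼠扶梯), placed on a card to switch ground mice into escalator movement.
; Init picks a full or low-health flipbook, and sphere traces or same-row box overlaps pass mice a sort value derived from the ladder's translucency.
; Tick keeps the tile's card collisions off and follows the card every 0.2 seconds.
; Once the card is invalid, it restores collision, cancels nearby mice's escalator movement and destroys itself.
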(event `self.Init`
  (params (bState :type Boolean) (Translucency :type Integer) (Location :type "Vector Structure") (CurCard :type "CardActor Object Reference"))
  (bind _returnvalue (`self.K2_GetActorLocation`))
  (`self.K2_SetActorLocation` (+ Location (0.0 18.0 5.0)))
  (if bState
    (`FlipbookBaseComponent.SetPlayAnimation` (`self.FlipbookBase`) "/Game/Resource/Texture/Sprite/VS/Sprite/Mouse/Mouse_1/普通/美味岛/修理鼠/FB_梯子满血.FB_梯子满血" false)
    (else
      (`FlipbookBaseComponent.SetPlayAnimation` (`self.FlipbookBase`) "/Game/Resource/Texture/Sprite/VS/Sprite/Mouse/Mouse_1/普通/美味岛/修理鼠/FB_梯子残血.FB_梯子残血" false)))
  (`FlipbookBaseComponent.SetTranslucency` (`self.FlipbookBase`) Translucency)
  (bind _output_get (set `self.Cur Card` CurCard))
  (bind _returnvalue_2 (`CardActor.GetUIMapMesh` _output_get))
  (set `self.UIMapMeshe` _returnvalue_2)
  (`self.InitTrans`)
  (`self.SetCardCollsionState` false)
  (bind _outhits (`KismetSystemLibrary.SphereTraceMulti` _returnvalue _returnvalue 15.0 "TraceTypeQuery4"))
  (for _array_element _outhits
    (bind _asnormal_base (cast `NormalBase` (`.HitActor` (`GameplayStatics.BreakHitResult` _array_element))))
    (`NormalBase.SetEscalatorMove` _asnormal_base (`self.NextTrans`) true)))

(event `self.ReceiveTick`
  (params (DeltaSeconds :type "Float (single-precision)"))
  (bind _returnvalue (`self.K2_GetActorLocation`))
  (bind _cur_card (`self.Cur Card`))
  (`self.SetCardCollsionState` false)
  (bind _returnvalue_2 (`UI_MapMeshe.GetLine` (`self.UIMapMeshe`)))
  (set `self.CurRow` (break `Line` _returnvalue_2))
  (bind _output_get (set `self.Delta Seconds` (+ (`self.Delta Seconds`) DeltaSeconds)))
  (if (> _output_get 0.2)
    (set `self.Delta Seconds` 0.0)
    (if (`KismetSystemLibrary.IsValid` _cur_card)
      (bind _returnvalue_3 (`CardActor.GetCurrentHP` _cur_card))
      (if (> _returnvalue_3 0.0)
        (`self.K2_SetActorLocation` (+ (`self.K2_GetActorLocation` _cur_card) (0.0 18.0 5.0))))
      (else
        (`self.SetCardCollsionState` true)
        (bind _outhits (`KismetSystemLibrary.SphereTraceMulti` _returnvalue _returnvalue 15.0 "TraceTypeQuery4"))
        (for _array_element _outhits
          (bind _asnormal_base (cast `NormalBase` (`.HitActor` (`GameplayStatics.BreakHitResult` _array_element))))
          (`NormalBase.SetEscalatorMove` _asnormal_base (`self.NextTrans`) false))
        (`self.K2_DestroyActor`)))))

(event `self.Box.OnComponentBeginOverlap`
  (params (OverlappedComponent :type "PrimitiveComponent Object Reference") (OtherActor :type "Actor Object Reference") (OtherComp :type "PrimitiveComponent Object Reference") (OtherBodyIndex :type Integer) (bFromSweep :type Boolean) (SweepResult :type "HitResult Structure (by ref)"))
  (bind _asnormal_base (cast `NormalBase` OtherActor))
  (bind _returnvalue (`MouseActor.GetMouseLine` _asnormal_base))
  (if (== (`self.CurRow`) (break `Line` _returnvalue))
    (bind _returnvalue_2 (`MouseActor.GetMouseLineType` _asnormal_base))
    (if (`|EnumEquality` _returnvalue_2 "OnGround")
      (`self.InitTrans`)
      (`NormalBase.SetEscalatorMove` _asnormal_base (`self.NextTrans`) true))))

(fn `InitTrans`
  (locals (MaxRow :type Integer) (MaxCol :type Integer) (Meshe :type "MesheControllComponent Object Reference"))
  (bind _returnvalue (`FlipbookBaseComponent.GetTranslucency` (`self.FlipbookBase`)))
  (if (== _returnvalue 0)
    (set `self.NextTrans` 980)
    (else
      (set `self.NextTrans` (- _returnvalue 59)))))

(fn `SetCardCollsionState`
  (params (bActive :type Boolean))
  (`KismetArrayLibrary.Array_Clear` (`self.Out All Cards`))
  (bind _outallcards (`UI_MapMeshe.GetAllCardsInstance` (`self.UIMapMeshe`)))
  (for _array_element _outallcards
    (`KismetArrayLibrary.Array_Add` (`self.Out All Cards`) _array_element)
    (`CardActor.SetCardCollisonState` _array_element bActive)))

(fn `UserConstructionScript`)