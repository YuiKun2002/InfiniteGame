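; Missile actor for the 轰隆隆 mouse boss.
; On spawn it waits out a first timeline, then calls InitLocation and drives UpdatePosition from a second timeline.
; Tick moves it upward along local Z until GetResult returns true.
; The impact logic (attack animation, flip, sphere trace killing cards, destroy on animation end) sits in unconnected nodes and never runs here.
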(event `self.ReceiveBeginPlay`
  (`Timeline|Timeline_0`
    (:`Finished`
      (`self.InitLocation`)
      (bind (_direction _newtrack_0) (`Timeline|Timeline_1`)
        (:`Update`
          (`self.UpdatePosition` _newtrack_0))))))

(event `self.ReceiveTick`
  (params (DeltaSeconds :type "Float (single-precision)"))
  (bind _returnvalue (`self.GetResult`))
  (if (not _returnvalue)
    (`self.K2_AddActorLocalOffset` (`KismetMathLibrary.MakeVector` 0.0 0.0 (* DeltaSeconds 200.0)))))

(fn `UserConstructionScript`)