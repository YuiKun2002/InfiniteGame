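; Bandage actor for the Pharaoh mouse boss, built as a mouse-type unit with a limited lifetime.
; Tick counts the Time variable down and, once it runs out, flags death a single time and calls SetMouseDeath.
; OnDeathed then runs MouseKill and destroys the actor.
; A flipbook animation call is present but left unconnected.
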(event `self.ReceiveBeginPlay`)

(event `self.ReceiveTick`
  (params (DeltaSeconds :type "Float (single-precision)"))
  (if (> (`self.time`) 0.0)
    (set `self.time` (- (`self.time`) DeltaSeconds))
    (elif (not (`self.bDeath`))
      (set `self.bDeath` true)
      (`self.SetMouseDeath` true))))

(event `self.OnDeathed`
  (`self.MouseKill`)
  (`self.K2_DestroyActor`))

(fn `UserConstructionScript`)