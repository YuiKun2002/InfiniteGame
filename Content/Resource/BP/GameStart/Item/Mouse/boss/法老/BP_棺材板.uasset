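; Coffin lid item for the pharaoh mouse boss that releases a mummy mouse onto its lane.
; SpawnBox stores the given mesh and location and takes the line from that mesh.
; The first animation-end callback sets Create; the next spawns the mummy mouse once, slightly below the stored location, guarded by Open.
; Defense and death events are empty, and their animation and collision logic is left unwired.
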(event `self.ReceiveBeginPlay`)

(event `self.SpawnBox`
  (params (CurMeshe :type "MapMeshe Object Reference") (CurLocation :type "Vector Structure"))
  (bind _output_get (set `self.Cur Meshe` CurMeshe))
  (set `self.Cur Location` CurLocation)
  (bind _returnvalue (`MapMeshe.GetLine` _output_get))
  (set `self.Line` _returnvalue))

(event `OnAnimationPlayEndBlueprint_1`
  (if (`self.bCreate`)
    (if (not (`self.bOpen`))
      (set `self.bOpen` true)
      (`MouseSpawnManager.MakeNewMouseByName` "/Game/Resource/BP/Data/MouseData/MouseData.MouseData" "木乃伊鼠" (`self.Line`) (+ (`self.Cur Location`) (0.0 0.0 -15.0))))
    (else
      (set `self.bCreate` true))))

(event `self.OnDefLowAnim`)

(event `self.OnDefAnim`)

(event `self.OnDeathed`)

(fn `UserConstructionScript`)