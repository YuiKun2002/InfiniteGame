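; BP_甲虫洞 is a beetle hole among the Pharaoh (法老) boss mouse assets, spawning beetle mice on its own grid cell.
; After init, a tick countdown creates a "甲虫" mouse from the data table every four seconds, slightly below the hole.
; A positive CallCount limits the spawns; the hole kills itself when that runs out or a spawn fails.
; Its death event also halts summoning.
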(event `self.ReceiveBeginPlay`
  ;[1 1 1] 初始化
  (`parent.ReceiveBeginPlay`)
  (add `self.OnInit` (delegate `Init`))
  ;[1 1 1] 召唤老鼠
  (add `self.Tick` (delegate `OnTick`)))

(event `OnTick` :!signature `self.Tick`
  (params (DeltaTime :type "Float (double-precision)"))
  ;[1 1 1] 召唤老鼠
  (if (`self.bInit_0`)
    (if (> (`self.Delta Seconds`) 0.0)
      (set `self.Delta Seconds` (- (`self.Delta Seconds`) DeltaTime))
      (else
        (set `self.Delta Seconds` 4.0)
        (bind _returnvalue (`self.GetMouseLine`))
        (bind _returnvalue_2 (`MouseSpawnManager.MakeNewMouseByName` "/Game/Resource/BP/Data/MouseData/MouseData.MouseData" "甲虫" (make `Line` (break `Line` _returnvalue) (`.Col` (break `Line` _returnvalue))) (+ (`self.K2_GetActorLocation`) (0.0 0.0 -15.0))))
        (if _returnvalue_2
          (if (> (`self.CallCount`) 0)
            (bind _output_get (set `self.CallCount` (- (`self.CallCount`) 1)))
            (if (<= _output_get 0)
              (`self.SetMouseDeath` true)
              (set `self.bInit_0` false)
              (clear `self.Tick`)))
          (else
            (`self.SetMouseDeath` true)
            (set `self.bInit_0` false)
            (clear `self.Tick`)))))))

(event `Init`
  ;[1 1 1] 初始化
  (set `self.bInit_0` true)
  (clear `self.OnInit`))

(event `self.OnDeathed`
  ;[1 1 1] 死亡
  (set `self.bInit_0` false))

(fn `UserConstructionScript`
  (`parent.UserConstructionScript`))