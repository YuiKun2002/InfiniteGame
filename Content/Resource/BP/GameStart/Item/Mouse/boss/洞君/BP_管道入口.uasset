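; Pipe entrance actor for the 洞君 mouse boss, placed on a map grid cell.
; Init snaps it to the map mesh at its Line row and column, copies that mesh's translucency sorting, and picks water or ground animations and offsets by line type.
; BeginPlay initializes rotation and fades it in through a timeline-driven material parameter.
; On water, the animation-end event reveals an extra sprite sorted one layer above.
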(event `self.OnAnimationPlayEndBlueprint`
  (if (`self.inWater`)
    (`SceneComponent.SetHiddenInGame` (`self.F_M_B_0_Ground_2`) false false)
    (`PrimitiveComponent.SetTranslucentSortPriority` (`self.F_M_B_0_Ground_2`) (+ (`self.Layer`) 1))))

(event `self.ReceiveBeginPlay`
  (`self.InitRotation`)
  (bind (_direction _newtrack_0) (`Timeline|Timeline_0` :!via `PlayFromStart`)
    (:`Update`
      (`MeshComponent.SetScalarParameterValueOnMaterials` (`self.M_Actor`) "A" (`KismetMathLibrary.Lerp` 0.0 1.0 _newtrack_0)))))

(fn `Init`
  (params (Line :type "Line Structure"))
  (locals (Ins :type "GameMapInstance Object Reference"))
  (bind (_line_row _line_col) (break `Line` (`local.Line`)))
  (bind _m_actor (`self.M_Actor`))
  (bind _returnvalue (`GameMapInstance.GetGameMapInstance`))
  (`/Engine/EditorBlueprintResources/StandardMacros.IsValid` _returnvalue
    (:`Is Valid`
      (bind _output_get (set `local.Ins` _returnvalue))
      (bind _returnvalue_2 (`MesheControllComponent.GetMapMesh` (`GameMapInstance.M_MesheControllComponent` _output_get) _line_row _line_col))
      (`self.K2_SetActorLocation` (`self.K2_GetActorLocation` _returnvalue_2))
      (set `self.Location` (`self.K2_GetActorLocation`))
      (bind _returnvalue_3 (`MapMeshe.GetTranslucency` _returnvalue_2))
      (`FlipbookBaseComponent.SetTranslucency` (`self.M_Actor`) _returnvalue_3)
      (bind _returnvalue_4 (`MapMeshe.GetLineType` _returnvalue_2))
      (bind _returnvalue_5 (`|EnumEquality` _returnvalue_4 "OnWater"))
      (if _returnvalue_5
        (`FlipbookBaseComponent.SetPlayAnimationOnce` _m_actor "/Game/Resource/Texture/Sprite/VS/Sprite/Mouse/Boss/0/Anim/F_M_B_0_Water_1.F_M_B_0_Water_1" "/Game/Resource/Texture/Sprite/VS/Sprite/Mouse/Boss/0/Anim/F_M_B_0_Water_2.F_M_B_0_Water_2")
        (set `self.inWater` _returnvalue_5)
        (set `self.Layer` _returnvalue_3)
        (`self.K2_SetActorLocation` (+ (`self.Location`) (0.018857 0.0 0.0)))
        (else
          (`FlipbookBaseComponent.SetPlayAnimationOnce` _m_actor "/Game/Resource/Texture/Sprite/VS/Sprite/Mouse/Boss/0/Anim/F_M_B_0_Ground_1.F_M_B_0_Ground_1" "/Game/Resource/Texture/Sprite/VS/Sprite/Mouse/Boss/0/Anim/F_M_B_0_Ground_2.F_M_B_0_Ground_2")
          (`self.K2_SetActorLocation` (+ (`self.Location`) (0.018857 0.0 -12.0))))))))

(fn `UserConstructionScript`)