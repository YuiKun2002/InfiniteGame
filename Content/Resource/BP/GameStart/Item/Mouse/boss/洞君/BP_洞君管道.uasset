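; Pipe Blueprint for the 洞君 mouse boss, managing a pipe entrance placed at a given map row and column.
; InitChannelin spawns BP_管道入口 and initializes it with that cell if none exists, and Destroyed removes it.
; An animation-end callback calls End when flagged, but the only logic setting that flag is disconnected.
; InitChannelOut, Hidde and hit reactions are empty, and the animation and fade logic never runs.
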(event `self.InitChannelIn`
  (params (NewLine :type "Line Structure"))
  (`/Engine/EditorBlueprintResources/StandardMacros.IsValid` (`self.InChannelActor`)
    (:`Is Valid`
      (set `self.bEnd` false))
    (:`Is Not Valid`
      (bind _returnvalue (`|SpawnActorFromClass` "/Game/Resource/BP/GameStart/Item/Mouse/boss/洞君/BP_管道入口.BP_管道入口_C" (`KismetMathLibrary.MakeTransform` (0.0 0.0 0.0)) "Undefined" "OverrideRootScale" null null))
      (`/Game/Resource/BP/GameStart/Item/Mouse/boss/洞君/BP_管道入口.Init` _returnvalue (make `Line` NewLine_Row NewLine_Col))
      (set `self.InChannelActor` _returnvalue)
      (set `self.bEnd` false))))

(event `self.InitChannelOut`
  (params (NewLine :type "Line Structure")))

(event `OnAnimationPlayEndBlueprint_1`
  (if (`self.bEnd`)
    (set `self.bEnd` false)
    (`self.End`)))

(event `self.Hidde`)

(event `self.BPBeHit`
  (params (CurHP :type "Float (single-precision)") (TotalHP :type "Float (single-precision)"))
  (if (> CurHP (* TotalHP 0.5))
    _))

(event `self.ReceiveDestroyed`
  (`self.K2_DestroyActor` (`self.InChannelActor`)))

(fn `UserConstructionScript`)