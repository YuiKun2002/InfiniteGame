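; Projectile template for the engineering vehicle mouse, lobbed at a grid position to damage the player's cards.
; Init stores the target, and a timeline moves the actor along a parabolic arc through a curve helper.
; On landing it damages cards that still have HP, killing and recording a destroyed one.
; The split animation, self-destruct and fallback sphere trace for cards sit in unconnected logic that never runs.
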(event `self.Init`
  (params (TargetLocation :type "Vector Structure (by ref)") (CurLocation :type "Vector Structure (by ref)") (TargetHitCard :type "Array of CardActor Object Reference (by ref)"))
  ;[1 1 1] 初始化条件以及位置信息
  (set `self.Target Location` TargetLocation)
  (set `self.Target Hit Card` TargetHitCard)
  (set `self.CurLocation` (`self.K2_GetActorLocation`))
  (set `self.bHit` false)
  ;[1 1 1] 从起始点飞向目标点的抛物线
  (bind (_direction _locationtime _highttime) (`Timeline|FlyTarget` :!via `PlayFromStart`)
    (:`Update`
      (bind _outlocation (`GameSystemFunction.GetCurveLineByTimeLineBlue` (`self.CurLocation`) (`self.Target Location`) 120.0 _locationtime _highttime))
      (`self.K2_SetActorLocation` _outlocation))
    (:`Finished`
      ;[1 1 1] 如果当前网格存在的卡片有效，则直接消耗血量，死亡则记录卡片损坏
      (for _array_element _
        (`/Engine/EditorBlueprintResources/StandardMacros.IsValid` _array_element
          (:`Is Valid`
            (bind _returnvalue (`CardActor.GetCurrentHP` _array_element))
            (if (> _returnvalue 0.0)
              (set `self.bHit` true)
              (bind _returnvalue_2 (`CardActor.UpdateCardState` _array_element (`self.ATK Value`) (`self.Up HP Value`)))
              (if _returnvalue_2
                (`CardActor.KillCard` _array_element)
                (`ResourceManagerComponent.ResourceAddBadCard`)
                (break)))))))))

(event `self.ReceiveBeginPlay`)

(fn `UserConstructionScript`)