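; Template Blueprint for the small magician mouse, which flies in an arc to a landing cell when spawned.
; On init it targets the map mesh at column 2 of its row, with a slight offset, and the Fly timeline moves it along a height curve.
; Timeline completion sets a flag, so the next animation end calls OnFlyEnd.
; Animation, attack-disable and collision-toggle nodes are left disconnected.
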(event `self.OnInitBlue`
  (`self.InitTargetLocation`)
  (bind (_direction _flytime _highttime) (`Timeline|Fly` :!via `PlayFromStart`)
    (:`Update`
      (bind _outlocation (`GameSystemFunction.GetCurveLineByTimeLineBlue` (`self.Cur Location`) (`self.Target Location`) (`self.Max Hight`) _flytime _highttime))
      (`self.K2_SetActorLocation` _outlocation))
    (:`Finished`
      (set `self.bPlayAnim` true))))

(event `OnAnimationPlayEndBlueprint_1`
  (if (`self.bPlayAnim`)
    (set `self.bPlayAnim` false)
    (`self.OnFlyEnd`)
    (`GameMapInstance.GetGameMapInstance`)))

(fn `InitTargetLocation`
  (set `self.Cur Location` (`self.K2_GetActorLocation`))
  (bind _returnvalue (`GameMapInstance.GetGameMapInstance`))
  (`/Engine/EditorBlueprintResources/StandardMacros.IsValid` _returnvalue
    (:`Is Valid`
      (bind _returnvalue_2 (`GameMapInstance.GetMesheControllComponent` _returnvalue))
      (bind _returnvalue_3 (`self.GetMouseLine`))
      (bind _returnvalue_4 (`MesheControllComponent.GetMapMesh` _returnvalue_2 (break `Line` _returnvalue_3) 2))
      (bind (_returnvalue_x _returnvalue_y _returnvalue_z) (`KismetMathLibrary.BreakVector` (`self.K2_GetActorLocation` _returnvalue_4)))
      (set `self.Target Location` (`KismetMathLibrary.MakeVector` _returnvalue_x (+ _returnvalue_y 15.0) (- _returnvalue_z 11.0)))
      (set `self.bPlayAnim` false))))

(fn `UserConstructionScript`)