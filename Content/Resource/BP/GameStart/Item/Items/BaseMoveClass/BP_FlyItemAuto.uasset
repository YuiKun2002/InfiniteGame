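; BP_FlyItemAuto is a pooled flying item that homes on a target through its AutoTrackShoot component.
; Init resets the component's location, starts tracking and zeroes a timer, while a hit or pool return stops tracking.
; Tick accumulates time while the component has no target and returns the item to the pool after a short grace period.
; Tick-while-paused on the component is disabled at init and re-enabled on return.
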(event `self.OnHit`
  (params (AttackType :type "EFlyItemAttackType Enum" :default "Def"))
  (`AutoTrackShootComponent.Stop` (`self.AutoTrackShoot`)))

(event `self.OnInit`
  (bind _autotrackshoot (`self.AutoTrackShoot`))
  (`ActorComponent.SetTickableWhenPaused` _autotrackshoot false)
  (`AutoTrackShootComponent.InitLocation` _autotrackshoot)
  (`AutoTrackShootComponent.Start` _autotrackshoot)
  (set `self.Delta Seconds` 0.0))

(event `self.OnReturn`
  (bind _autotrackshoot (`self.AutoTrackShoot`))
  (`ActorComponent.SetTickableWhenPaused` _autotrackshoot true)
  (`AutoTrackShootComponent.Stop` _autotrackshoot))

(event `self.ReceiveTick`
  (params (DeltaSeconds :type "Float (single-precision)"))
  (bind _returnvalue (`AutoTrackShootComponent.GetTarget` (`self.AutoTrackShoot`)))
  (if _returnvalue
    (set `self.Delta Seconds` 0.0)
    (else
      (bind _output_get (set `self.Delta Seconds` (+ (`self.Delta Seconds`) DeltaSeconds)))
      (if (>= _output_get 0.3)
        (`self.ReturnPool`)))))

(fn `UserConstructionScript`)