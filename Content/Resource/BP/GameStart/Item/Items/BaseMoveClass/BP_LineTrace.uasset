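; BP_LineTrace is a pooled item move class that hits MouseActor targets along a straight line.
; MakeLineDrection sets the pool return time, then multi-traces Pawn objects from the actor's location along a Y/Z offset, ignoring the map mesh and card actor.
; Each hit that casts to MouseActor is passed to HitMouseOverlapBegin, reusing the overlap hit handler.
; The trace leaves its debug line drawn for a duration.
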(fn `MakeLineDrection`
  (params (XDirection :type "Float (double-precision)" :default 290.0) (YDirection :type "Float (double-precision)") (LifeSpawnTime :type "Float (double-precision)" :default 0.66))
  (bind _returnvalue (`self.K2_GetActorLocation`))
  (`self.SetReturnPoolTime` LifeSpawnTime)
  (bind _returnvalue_2 (`GameplayStatics.GetActorOfClass` "/Game/Resource/BP/GameStart/VS/AMapMeshe.AMapMeshe_C"))
  (bind _returnvalue_3 (`GameplayStatics.GetActorOfClass` "/Script/FVM.CardActor"))
  (bind (_outhits _returnvalue_4) (`KismetSystemLibrary.LineTraceMultiForObjects` _returnvalue (+ _returnvalue (`KismetMathLibrary.MakeVector` 0.0 XDirection YDirection)) (`|MakeArray` "ObjectTypeQuery3" :!type "EObjectTypeQuery Enum") false (`|MakeArray` _returnvalue_2 _returnvalue_3 :!type "Actor Object Reference") "ForDuration"))
  (if _returnvalue_4
    (for _array_element _outhits
      (bind _asmouse_actor (cast `MouseActor` (`.HitActor` (`GameplayStatics.BreakHitResult` _array_element))))
      (`self.HitMouse_OverlapBegin` _asmouse_actor))))

(fn `UserConstructionScript`)