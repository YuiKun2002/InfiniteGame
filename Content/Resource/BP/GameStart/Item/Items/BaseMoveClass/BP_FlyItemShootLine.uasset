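; BP_FlyItemShootLine is a flying-item movement class for straight-line shots that can hit targets on water, underwater and on land.
; On BeginPlay it passes MoveMode to the ShootLine component as its move node.
; OnInit enables movement and OnReturn disables it, each also toggling tick-when-paused inversely to movement.
; On hit, movement stops unless the attack type is Panetrate, so penetrating shots keep flying.
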(event `self.ReceiveBeginPlay`
  ;[1 1 1] 直线模式( 能打击水上水下陆地)
  (set `ShootLineComponent.M_MoveNode` (`self.MoveMode`) (`self.ShootLine`)))

(event `self.OnInit`
  ;[1 1 1] 直线模式( 能打击水上水下陆地)
  (`ShootLineComponent.SetMoveEnabled` (`self.ShootLine`) true)
  (`ActorComponent.SetTickableWhenPaused` (`self.ShootLine`) false))

(event `self.OnReturn`
  ;[1 1 1] 直线模式( 能打击水上水下陆地)
  (`ShootLineComponent.SetMoveEnabled` (`self.ShootLine`) false)
  (`ActorComponent.SetTickableWhenPaused` (`self.ShootLine`) true))

(event `self.OnHit`
  (params (AttackType :type "EFlyItemAttackType Enum" :default "Def"))
  ;[1 1 1] 直线模式( 能打击水上水下陆地)
  (if (not (`|EnumEquality` AttackType "Panetrate"))
    (`ShootLineComponent.SetMoveEnabled` (`self.ShootLine`) false)))

(fn `UserConstructionScript`)