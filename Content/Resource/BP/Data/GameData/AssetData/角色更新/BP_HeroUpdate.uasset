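; BP_HeroUpdate is a data update step that creates or refreshes the player's saved hero roster.
; Its Update event first checks net mode, which can end the step without changes.
; Player data with no valid item ID gets a default set of named heroes, with Explorer as current.
; Existing data runs its hero list through UpdatePlayerData; both paths save the player data, and every branch calls ExecFinish.
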(event `PlayerUpdateClassInterface.Update`
  (params (PlayerDataIns :type "PlayerStructManager Object Reference"))
  (if (`GameCacheSubsystem.GetNetMode`)
    (`self.ExecFinish`)
    (elif (== (`.M_ItemID` (break `ItemHeroBase` (`PlayerStructManager.PlayerData` PlayerDataIns))) -1)
      (bind _output_get (set `PlayerStructManager.PlayerData` (`ItemHeroDataFunc.CreateNewPlayerData` "Explorer" 12) PlayerDataIns))
      (set `PlayerStructManager.M_PlayerItems_Heroes` (`|MakeArray` _output_get (`ItemHeroDataFunc.CreateNewPlayerData` "Jingke" 13) (`ItemHeroDataFunc.CreateNewPlayerData` "Lilith" 14) (`ItemHeroDataFunc.CreateNewPlayerData` "Bustre" 15) (`ItemHeroDataFunc.CreateNewPlayerData` "Jputier" 16) (`ItemHeroDataFunc.CreateNewPlayerData` "Icywing" 17) (`ItemHeroDataFunc.CreateNewPlayerData` "Zeta" 18)) PlayerDataIns)
      (`GameSystemFunction.SaveCurrentPlayerData` "新增保存的角色")
      (`self.ExecFinish`)
      (else
        (set `PlayerStructManager.M_PlayerItems_Heroes` (`ItemHeroDataFunc.UpdatePlayerData` (`PlayerStructManager.M_PlayerItems_Heroes` PlayerDataIns)) PlayerDataIns)
        (`GameSystemFunction.SaveCurrentPlayerData` "更新角色数据表")
        (`self.ExecFinish`)))))