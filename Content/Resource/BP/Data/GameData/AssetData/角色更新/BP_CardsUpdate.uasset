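; Player-data update Blueprint that seeds a player's card item list with a default set of cards.
; Its Update event acts only when MPlayerItemsCard on the passed player data is empty, so existing lists are left untouched.
; A Sequence node appends the predefined card variables in small batches, with no other logic or per-card checks.
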(event `PlayerUpdateClassInterface.Update`
  (params (PlayerDataIns :type "PlayerStructManager Object Reference"))
  (bind _m_playeritems_card (`PlayerStructManager.M_PlayerItems_Card` PlayerDataIns))
  (if (== (`KismetArrayLibrary.Array_Length` _m_playeritems_card) 0)
    (`|ExecutionSequence`
      (:`then_0`
        (`KismetArrayLibrary.Array_Add` _m_playeritems_card (`self.NewVar_0`))
        (`KismetArrayLibrary.Array_Add` _m_playeritems_card (`self.NewVar_1`))
        (`KismetArrayLibrary.Array_Add` _m_playeritems_card (`self.NewVar_2`))
        (`KismetArrayLibrary.Array_Add` _m_playeritems_card (`self.NewVar_3`)))
      (:`then_1`
        (`KismetArrayLibrary.Array_Add` _m_playeritems_card (`self.NewVar_4`))
        (`KismetArrayLibrary.Array_Add` _m_playeritems_card (`self.NewVar_5`))
        (`KismetArrayLibrary.Array_Add` _m_playeritems_card (`self.NewVar_6`))
        (`KismetArrayLibrary.Array_Add` _m_playeritems_card (`self.NewVar_7`)))
      (:`then_2`
        (`KismetArrayLibrary.Array_Add` _m_playeritems_card (`self.NewVar_8`))
        (`KismetArrayLibrary.Array_Add` _m_playeritems_card (`self.NewVar_9`))
        (`KismetArrayLibrary.Array_Add` _m_playeritems_card (`self.NewVar_10`))
        (`KismetArrayLibrary.Array_Add` _m_playeritems_card (`self.NewVar_11`)))
      (:`then_3`
        (`KismetArrayLibrary.Array_Add` _m_playeritems_card (`self.NewVar_12`))
        (`KismetArrayLibrary.Array_Add` _m_playeritems_card (`self.NewVar_13`))
        (`KismetArrayLibrary.Array_Add` _m_playeritems_card (`self.NewVar_14`))
        (`KismetArrayLibrary.Array_Add` _m_playeritems_card (`self.NewVar_15`)))
      (:`then_4`
        (`KismetArrayLibrary.Array_Add` _m_playeritems_card (`self.NewVar_16`))
        (`KismetArrayLibrary.Array_Add` _m_playeritems_card (`self.NewVar_17`))
        (`KismetArrayLibrary.Array_Add` _m_playeritems_card (`self.NewVar_18`))
        (`KismetArrayLibrary.Array_Add` _m_playeritems_card (`self.NewVar_19`)))
      (:`then_5`
        (`KismetArrayLibrary.Array_Add` _m_playeritems_card (`self.NewVar_20`))
        (`KismetArrayLibrary.Array_Add` _m_playeritems_card (`self.NewVar_21`))
        (`KismetArrayLibrary.Array_Add` _m_playeritems_card (`self.NewVar_22`))
        (`KismetArrayLibrary.Array_Add` _m_playeritems_card (`self.NewVar_23`)))
      (:`then_6`
        (`KismetArrayLibrary.Array_Add` _m_playeritems_card (`self.NewVar_24`))
        (`KismetArrayLibrary.Array_Add` _m_playeritems_card (`self.NewVar_25`))
        (`KismetArrayLibrary.Array_Add` _m_playeritems_card (`self.NewVar_26`))
        (`KismetArrayLibrary.Array_Add` _m_playeritems_card (`self.NewVar_27`)))
      (:`then_7`
        (`KismetArrayLibrary.Array_Add` _m_playeritems_card (`self.NewVar_28`))
        (`KismetArrayLibrary.Array_Add` _m_playeritems_card (`self.NewVar_29`))
        (`KismetArrayLibrary.Array_Add` _m_playeritems_card (`self.NewVar_30`))
        (`KismetArrayLibrary.Array_Add` _m_playeritems_card (`self.NewVar_31`))
        (`KismetArrayLibrary.Array_Add` _m_playeritems_card (`self.NewVar_32`))))))