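; Network helper Blueprint that builds HTTP endpoint URLs for the game's backend API: accounts, coins, player bag and shop.
; Each getter appends a route to GetBaseURL, which hardcodes a LAN host and port.
; Coin and bag URLs also append the player ID from PlayerDataSubsystem as a userId query.
; Prescription and ATK card getters are empty stubs, and the sign-in getter returns only the base URL.
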(fn `GetATKCardsURL`)

(fn `GetBaseURL`
  (returns (BaseURL :type String))
  (return (`KismetStringLibrary.Concat_StrStr` "http://" "192.168.0.101" ":" "8888" "/api/")))

(fn `GetCoinURL`
  (returns (URL :type String))
  (return (`KismetStringLibrary.Concat_StrStr` (`KismetStringLibrary.Concat_StrStr` (`self.GetBaseURL` null) "money/getMoney?userId=") (`PlayerStructManager.GetPlayerID` (`PlayerDataSubsystem.GetPlayerDataInstance` (subsystem `PlayerDataSubsystem`))))))

(fn `GetLoginURL`
  (returns (URL :type String))
  (return (`KismetStringLibrary.Concat_StrStr` (`self.GetBaseURL` null) "user/login")))

(fn `GetLogoutURL`
  (returns (URL :type String))
  (return (`KismetStringLibrary.Concat_StrStr` (`self.GetBaseURL` null) "user/logout")))

(fn `GetPlayerBagURL`
  (returns (ReturnValue :type String))
  (return (`KismetStringLibrary.Concat_StrStr` (`KismetStringLibrary.Concat_StrStr` (`self.GetBaseURL` null) "package/getPackageItems?userId=") (`PlayerStructManager.GetPlayerID` (`PlayerDataSubsystem.GetPlayerDataInstance` (subsystem `PlayerDataSubsystem`))))))

(fn `GetPrescriptionURL`)

(fn `GetRegisterURL`
  (returns (URL :type String))
  (return (`KismetStringLibrary.Concat_StrStr` (`self.GetBaseURL` null) "user/register")))

(fn `GetShopURL`
  (returns (URL :type String))
  (return (`KismetStringLibrary.Concat_StrStr` (`self.GetBaseURL` null) "item/queryAllItem")))

(fn `GetSigninURL`
  (returns (URL :type String))
  (return (`KismetStringLibrary.Concat_StrStr` (`self.GetBaseURL` null))))

(fn `GetUpdateURL`
  (returns (URL :type String))
  (return (`KismetStringLibrary.Concat_StrStr` (`self.GetBaseURL` null) "user/update")))