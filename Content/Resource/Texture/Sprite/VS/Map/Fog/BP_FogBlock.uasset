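; BP_FogBlock is a map fog block that fades its plane in and out on request.
; A DisplayBlock dispatcher drives the Show timeline, which animates material scalar "A" and hides the block after fading out.
; TimeDispaly clears the fog temporarily, using Tick as a countdown enabled only until it restores visibility from GetDisplayResult.
; SetTrans sets the plane's translucent sort priority for layering.
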(event `self.ReceiveBeginPlay`
  ;[1 1 1] 绑定核心功能，迷雾的显示和消失
  (`self.SetActorTickEnabled` false)
  (`self.SetActorHiddenInGame` true)
  (`SceneComponent.SetHiddenInGame` (`self.Plane`) true false)
  (add `self.DisplayBlock` (delegate `DisBlock`)))

(event `DisBlock` :!signature `self.DisplayBlock`
  (params (Value :type Boolean))
  ;[1 1 1] 绑定核心功能，迷雾的显示和消失
  (if Value
    (`SceneComponent.SetHiddenInGame` (`self.Plane`) false false)
    (`self.SetActorHiddenInGame` false)
    (bind (_direction _value) (`Timeline|Show` :!label _label)
      (:`Update`
        (`MeshComponent.SetScalarParameterValueOnMaterials` (`self.Plane`) "A" _value))
      (:`Finished`
        (if (not Value)
          (`self.SetActorHiddenInGame` true)
          (`SceneComponent.SetHiddenInGame` (`self.Plane`) true false))))
    (else
      (goto _label :!via `Reverse`))))

(event `self.Dispaly`
  (params (Value :type Boolean))
  ;[1 1 1] 事件触发，调用迷雾功能
  (`self.DisplayBlock` Value))

(event `self.SetTrans`
  (params (Trans :type Integer))
  ;[1 1 1] 渲染层级设置
  (`PrimitiveComponent.SetTranslucentSortPriority` (`self.Plane`) Trans))

(event `self.TimeDispaly`
  (params (time :type "Float (single-precision)"))
  ;[0.968 1 0.441] 时间显示
  ;;[1 1 1] 事件触发【迷雾消失，一段时间后根据情况显示】
  (`self.DisplayBlock` false)
  (set `self.Time` time)
  (`self.SetActorTickEnabled` true))

(event `self.ReceiveTick`
  (params (DeltaSeconds :type "Float (single-precision)"))
  ;[0.968 1 0.441] 时间显示
  ;;[1 1 1] 实现逻辑
  (if (> (`self.Time`) 0.0)
    (set `self.Time` (- (`self.Time`) DeltaSeconds))
    (else
      (`self.SetActorTickEnabled` false)
      (bind _returnvalue (`self.GetDisplayResult`))
      (`self.DisplayBlock` _returnvalue))))

(fn `UserConstructionScript`
  (`MeshComponent.SetScalarParameterValueOnMaterials` (`self.Plane`) "A" 0.0))